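; BP_Spirit_001 is a spirit VFX actor whose cube turns to watch the player character.
; BeginPlay spawns the NS_Cloud_001 Niagara system at the Scene component's location.
; Each Tick casts the main controller's pawn to BP_PlayedCharacter and applies a world-space look-at toward its mesh as the Cube's relative rotation.
; An NS_Eye spawn and a whole-actor rotation variant are left unconnected.
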(event EventBeginPlay
  (Niagara|SpawnSystematLocation "/Game/VFX/NS_Cloud_001.NS_Cloud_001" (Transformation|GetWorldLocation (Variables|Default|GetScene))))

(event EventTick
  (params (DeltaSeconds :type Float%20%28single-precision%29))
  (bind _cube (Variables|Default|GetCube))
  (bind _asbp_played_character (Utilities|Casting|CastToBP_PlayedCharacter (Pawn|GetControlledPawn (CallFunction|GetMainPlayerController))))
  (Transformation|SetRelativeRotation _cube (Math|Rotator|FindLookatRotation (Transformation|GetWorldLocation _cube) (Transformation|GetWorldLocation (Variables|/Script/Engine.Character|GetMesh _asbp_played_character))) false false))

(fn ConstructionScript)
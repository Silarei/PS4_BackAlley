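; BP_TestRitualScene is a scripted ritual scene event that takes control of the player and stages a cinematic moment.
; When triggered by the played character, it enters cinematic mode and disables gravity, capsule collision and head bob.
; One timeline turns the view toward a rotation target, then a second moves the character to a location target.
; On arrival, the main player controller plays the nail-and-cards animation.
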(event EventBeginPlay)

(event EventThisEventBehavior
  (params (OtherComp :type Primitive%20Component%20Object%20Reference))
  (bind _mainplayercontroller (CallFunction|GetMainPlayerController))
  (bind _playerlocationtarget (Variables|Default|GetPlayerLocationTarget))
  (bind _returnvalue (Transformation|GetWorldLocation _playerlocationtarget))
  (bind _asbp_played_character (Utilities|Casting|CastToBP_PlayedCharacter (Components|GetOwner OtherComp)))
  (Variables|Default|SetPlayedCharacter _asbp_played_character)
  (Default|EnterCinematicMode _mainplayercontroller)
  (Variables|Default|SetBaseRotation (Pawn|GetControlRotation _mainplayercontroller :!class /Script/Engine.Controller))
  (Physics|SetEnableGravity (Variables|/Script/Engine.Character|GetCapsuleComponent (Variables|Default|GetPlayedCharacter)) false)
  (Collision|SetCollisionEnabled (Variables|/Script/Engine.Character|GetCapsuleComponent (Variables|Default|GetPlayedCharacter)) "NoCollision")
  (Default|DisableHeadBob (Variables|Default|GetPlayedCharacter))
  (bind _rotation (Timeline|FirstLookAtCorpse PlayFromStart)
    (:Update
      (Pawn|SetControlRotation _mainplayercontroller (Math|Rotator|Lerp(Rotator) (Variables|Default|GetBaseRotation) (Math|Rotator|FindLookatRotation (Transformation|GetWorldLocation (Variables|/Game/Blueprints/BP_PlayedCharacter.BP_PlayedCharacter_C|GetFirstPersonCamera (Variables|Default|GetPlayedCharacter))) (Transformation|GetWorldLocation (Variables|Default|GetPlayerRotationTarget))) _rotation true))
      (if (Math|Rotator|Equal(Rotator) (Pawn|GetControlRotation (CallFunction|GetMainPlayerController) :!class /Script/Engine.Controller) (Math|Rotator|FindLookatRotation (Transformation|GetWorldLocation (Variables|/Game/Blueprints/BP_PlayedCharacter.BP_PlayedCharacter_C|GetFirstPersonCamera (Variables|Default|GetPlayedCharacter))) (Transformation|GetWorldLocation (Variables|Default|GetPlayerRotationTarget))) 0.0001)
        (Audio|Components|Audio|Stop (Variables|Default|GetFirstLookAtCorpse))
        (bind _alpha (Timeline|MoveTowards PlayFromStart)
          (:Update
            (Transformation|SetActorLocation (Variables|Default|GetPlayedCharacter) (Math|Vector|Lerp(Vector) (Transformation|GetActorLocation (Variables|Default|GetPlayedCharacter)) _returnvalue _alpha) false false)
            (if (< (Math|Vector|Distance(Vector) (Transformation|GetActorLocation (Variables|Default|GetPlayedCharacter)) _returnvalue) 0.001)
              (Audio|Components|Audio|Stop (Variables|Default|GetMoveTowards))
              (Variables|Default|SetBaseRotation (Pawn|GetControlRotation (CallFunction|GetMainPlayerController) :!class /Script/Engine.Controller))
              (Default|PlayNailandCardsAnim (CallFunction|GetMainPlayerController)))))))))

(fn ConstructionScript)
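; Interactable door that the player swings open or shut by holding the interact input and turning the character.
; While selected, it shows an interaction icon and ticks DragDoor, then clamps door yaw between zero and MaxAngle.
; DragDoor scales turn rate by Sensitivity and the character's forward X or Y, choosing axis and sign from the root's world yaw.
; Releasing the input or the player leaving the Box ends the drag.
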(event OnComponentEndOverlap(Box)
  (params (OverlappedComponent :type Primitive%20Component%20Object%20Reference) (OtherActor :type Actor%20Object%20Reference) (OtherComp :type Primitive%20Component%20Object%20Reference) (OtherBodyIndex :type Integer))
  (if (== OtherActor (Variables|/Game/Blueprints/BP_MainPlayerController.BP_MainPlayerController_C|GetPlayed_Character (Variables|Default|GetMain%20Player%20Controller)))
    (Variables|Default|SetisHoldingLMB false)))

(event EventBeginPlay
  (|CallParentFunction) ; This node is disabled and will not be called.\nDrag off pins to build functionality.
)

(event EventTick
  (params (DeltaSeconds :type Float%20%28single-precision%29))
  (bind _door (Variables|Default|GetDoor))
  (bind _door_2 (Variables|Default|GetDoor))
  (bind _relativerotation (Variables|/Script/Engine.SceneComponent|GetRelativeRotation _door))
  (bind _relativerotation_2 (Variables|/Script/Engine.SceneComponent|GetRelativeRotation _door_2))
  (Utilities|FlowControl|Sequence
    (:then_0
      (|DragDoor))
    (:then_1
      (if (<= (.yaw _relativerotation) 0.0)
        (Transformation|SetRelativeRotation _door (Math|Rotator|MakeRotator (.roll _relativerotation) (.pitch _relativerotation) 0.0) false false)))
    (:then_2
      (if (>= (.yaw _relativerotation_2) (Variables|Default|GetMaxAngle))
        (Transformation|SetRelativeRotation _door_2 (Math|Rotator|MakeRotator (.roll _relativerotation_2) (.pitch _relativerotation_2) (Variables|Default|GetMaxAngle)) false false)))))

(event EventInterractPressed
  (Variables|Default|SetisHoldingLMB true))

(event EventInterractReleased
  (Variables|Default|SetisHoldingLMB false))

(fn ConstructionScript
  (|CallParentFunction)
  (Transformation|AttachComponentToComponent (Variables|Default|GetInteractionWidget) (Variables|Default|GetDoor) "None" "KeepRelative" "KeepRelative" "KeepRelative" true))

(fn OnUnselected
  (|CallParentFunction)
  (Actor|Tick|SetActorTickEnabled false)
  (CallFunction|HideIcon (Variables|Default|GetInteractionWidget1)))

(fn OnSelected
  (|CallParentFunction)
  (Actor|Tick|SetActorTickEnabled true)
  (CallFunction|ShowIcon (Variables|Default|GetInteractionWidget1)))
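; Interactable narrative object that the player can bring in front of the first-person camera and rotate for inspection.
; Interacting toggles inspect mode, which moves the mesh ahead of the camera, disables player movement and binds the player controller's turn dispatchers to yaw and roll the mesh in world space.
; Interacting again restores the transform saved at BeginPlay, unbinds those dispatchers and re-enables movement.
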(event Custom|ExitTurningMode
  (bind _staticmesh (Variables|Default|GetStaticMesh))
  (bind _main_player_controller (Variables|Default|GetMain%20Player%20Controller))
  (Transformation|SetWorldLocation _staticmesh (Variables|Default|GetOriginalLocation) false false)
  (Transformation|SetRelativeRotation _staticmesh (Variables|Default|GetOriginalRotation) false false)
  (Default|UnbindAllfromTurnObjectRight _main_player_controller)
  (Default|UnbindAllfromTurnObjectUp _main_player_controller)
  (Default|EnableMovement _main_player_controller))

(event Custom|TurnObjectRight
  (params (Delta%20Rotation%20Z%20%28Yaw%29 :type Float%20%28single-precision%29))
  (Transformation|AddWorldRotation (Variables|Default|GetStaticMesh) (Math|Rotator|MakeRotator 0.0 0.0 Delta%20Rotation%20Z%20%28Yaw%29) false false))

(event Custom|TurnObjectUp
  (params (Delta%20Rotation%20X%20%28Roll%29 :type Float%20%28single-precision%29))
  (Transformation|AddWorldRotation (Variables|Default|GetStaticMesh) (Math|Rotator|MakeRotator Delta%20Rotation%20X%20%28Roll%29 0.0 0.0) false false))

(event EventBeginPlay
  (bind _staticmesh (Variables|Default|GetStaticMesh))
  (|CallParentFunction)
  (Variables|Default|SetOriginalLocation (Transformation|GetWorldLocation _staticmesh))
  (Variables|Default|SetOriginalRotation (Variables|/Script/Engine.SceneComponent|GetRelativeRotation _staticmesh)))

(event EventInterractPressed
  (bind _playedcharacter (CallFunction|GetPlayedCharacter))
  (bind _main_player_controller (Variables|Default|GetMain%20Player%20Controller))
  (bind _firstpersoncamera (Variables|/Game/Blueprints/BP_PlayedCharacter.BP_PlayedCharacter_C|GetFirstPersonCamera _playedcharacter))
  (if (Variables|Default|GetIsInMoveMode)
    (Variables|Default|SetIsInMoveMode false)
    (CallFunction|ExitTurningMode)
    (else
      (Variables|Default|SetIsInMoveMode true)
      (Transformation|SetWorldLocation (Variables|Default|GetStaticMesh) (+ (Transformation|GetWorldLocation _firstpersoncamera) (* (Math|Vector|GetForwardVector _firstpersoncamera) (Variables|Default|GetDistanceFromCamera))) false false)
      (Default|DisableMovement _main_player_controller)
      (Default|BindOncetoTurnObjectRight _main_player_controller (EventDispatchers|CreateEvent :!event Custom|TurnObjectRight))
      (Default|BindOncetoTurnObjectUp _main_player_controller (EventDispatchers|CreateEvent :!event Custom|TurnObjectUp)))))

(fn ConstructionScript
  (|CallParentFunction))
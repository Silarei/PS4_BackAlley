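; End-game ritual scene that locks the player into a cinematic look at a corpse while a phone buzzes.
; With two or more essential items it shows WBP_EndChoice; otherwise it auto-triggers PickUp, which plays bad-ending dialogue and quits.
; UseTarot moves the player into place and plays two-arm montages, then quits.
; Montage notifies spawn, socket-attach and release the tarot box, cards, hammer and nail, with timelines driving movement.
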(event Custom|MainAnim
  (bind _playedcharacter (Variables|Default|GetPlayedCharacter))
  (bind _playedcharacter_2 (Variables|Default|GetPlayedCharacter))
  (bind _cardlocation1 (Variables|Default|GetCardLocation1))
  (bind _cardlocation2 (Variables|Default|GetCardLocation2))
  (bind _cardlocation3 (Variables|Default|GetCardLocation3))
  (bind _rightarm (Variables|/Game/Blueprints/BP_PlayedCharacter.BP_PlayedCharacter_C|GetRightArm _playedcharacter_2))
  (bind _mesh (Variables|/Script/Engine.Character|GetMesh _playedcharacter))
  (Default|SetArmsVisibility (Variables|Default|GetPlayedCharacter) true)
  (Components|Animation|SetAnimation _rightarm "/Game/Animations/Test/AM_R_CardNail_Anim.AM_R_CardNail_Anim")
  (Components|Animation|SetAnimation _mesh "/Game/Animations/Test/A_LeftArmCardNail_003.A_LeftArmCardNail_003")
  (bind _notifyname (Animation|Montage|PlayMontage _rightarm "/Game/Animations/Test/AM_R_CardNail_Anim.AM_R_CardNail_Anim")
    (:then
      (bind _returnvalue (Game|SpawnActorfromClass "/Game/Blueprints/EndSequence/BP_TarotBox.BP_TarotBox_C" (Math|Transform|MakeTransform "0, 0, 0" "0, 0, 0" "0.500000,0.500000,0.500000") "Undefined" 0 0))
      (bind _output_get (Variables|Default|SetTarotBox _returnvalue))
      (Transformation|AttachComponentToComponent _output_get (Variables|/Script/Engine.Character|GetMesh (Variables|Default|GetPlayedCharacter)) "CardBoxSocket" "KeepRelative" "KeepRelative" "KeepRelative" true)
      (bind _notifyname_2 (Animation|Montage|PlayMontage _mesh "/Game/Animations/Test/AM_L_CardNail_Anim.AM_L_CardNail_Anim")
        (:OnCompleted
          (Default|SetArmsVisibility (Variables|Default|GetPlayedCharacter) false)
          (Game|QuitGame 0 "Quit" false))
        (:OnNotifyBegin
          (if (Utilities|Name|Equal(Name) _notifyname_2 (Utilities|Name|MakeLiteralName "DestroyTarot"))
            (Transformation|DetachFromActor (Variables|Default|GetTarotBox) "KeepRelative" "KeepRelative" "KeepRelative")
            (Actor|DestroyActor (Variables|Default|GetTarotBox))
            (elif (Utilities|Name|Equal(Name) _notifyname_2 (Utilities|Name|MakeLiteralName "AddNail"))
              (bind _returnvalue_2 (Game|SpawnActorfromClass "/Game/Blueprints/EndSequence/BP_Nail.BP_Nail_C" (Math|Transform|MakeTransform "0, 0, 0" "0, 0, 0" "0.500000,0.500000,0.500000") "Undefined" 0 0))
              (bind _output_get_2 (Variables|Default|SetNail _returnvalue_2))
              (Transformation|AttachComponentToComponent _output_get_2 (Variables|/Script/Engine.Character|GetMesh (Variables|Default|GetPlayedCharacter)) "NailSocket" "KeepRelative" "KeepRelative" "KeepRelative" true)
              (elif (Utilities|Name|Equal(Name) _notifyname_2 (Utilities|Name|MakeLiteralName "ReleaseNail"))
                (Transformation|DetachFromActor (Variables|Default|GetNail) "KeepWorld" "KeepWorld" "KeepWorld")
                (elif (Utilities|Name|Equal(Name) _notifyname_2 (Utilities|Name|MakeLiteralName "MoveNail"))
                  (CallFunction|MoveNail))))))))
    (:OnNotifyBegin
      (if (Utilities|Name|Equal(Name) _notifyname (Utilities|Name|MakeLiteralName "AddCard1"))
        (bind _returnvalue_3 (Game|SpawnActorfromClass "/Game/Blueprints/EndSequence/BP_TarotCard.BP_TarotCard_C" (Math|Transform|MakeTransform "0, 0, 0" "0.000000, 0,90.000000" "0.500000,0.500000,0.500000") "Undefined" 0 0))
        (Variables|Default|SetCard1 _returnvalue_3)
        (Transformation|AttachComponentToComponent (Variables|Default|GetCard1) (Variables|/Game/Blueprints/BP_PlayedCharacter.BP_PlayedCharacter_C|GetRightArm (Variables|Default|GetPlayedCharacter)) "CardSocket" "KeepRelative" "KeepRelative" "KeepWorld" true)
        (elif (Utilities|Name|Equal(Name) _notifyname (Utilities|Name|MakeLiteralName "ReleaseCard1"))
          (Transformation|DetachFromActor (Variables|Default|GetCard1) "KeepRelative" "KeepRelative" "KeepRelative")
          (Transformation|SetWorldScale3D (Variables|/Game/Blueprints/EndSequence/BP_TarotCard.BP_TarotCard_C|GetDefaultSceneRoot (Variables|Default|GetCard1)) "1.000000,1.000000,1.000000")
          (Transformation|AddActorLocalRotation (Variables|Default|GetCard1) "0.000000,0.000000,-90.000000" false false)
          (Transformation|SetWorldLocationAndRotation (Variables|/Game/Blueprints/EndSequence/BP_TarotCard.BP_TarotCard_C|GetDefaultSceneRoot (Variables|Default|GetCard1)) (Transformation|GetWorldLocation _cardlocation1) (Transformation|GetWorldRotation _cardlocation1) false false)
          (elif (Utilities|Name|Equal(Name) _notifyname (Utilities|Name|MakeLiteralName "AddCard2"))
            (bind _returnvalue_4 (Game|SpawnActorfromClass "/Game/Blueprints/EndSequence/BP_TarotCard.BP_TarotCard_C" (Math|Transform|MakeTransform "0, 0, 0" "0, 0,90.000000" "0.500000,0.500000,0.500000") "Undefined" 0 0))
            (bind _output_get_3 (Variables|Default|SetCard2 _returnvalue_4))
            (Transformation|AttachComponentToComponent _output_get_3 (Variables|/Game/Blueprints/BP_PlayedCharacter.BP_PlayedCharacter_C|GetRightArm (Variables|Default|GetPlayedCharacter)) "CardSocket" "KeepRelative" "KeepRelative" "KeepWorld" true)
            (elif (Utilities|Name|Equal(Name) _notifyname (Utilities|Name|MakeLiteralName "ReleaseCard2"))
              (Transformation|DetachFromActor (Variables|Default|GetCard2) "KeepRelative" "KeepRelative" "KeepRelative")
              (Transformation|SetWorldScale3D (Variables|/Game/Blueprints/EndSequence/BP_TarotCard.BP_TarotCard_C|GetDefaultSceneRoot (Variables|Default|GetCard2)) "1.000000,1.000000,1.000000")
              (Transformation|AddActorLocalRotation (Variables|Default|GetCard2) "0.000000,0.000000,-90.000000" false false)
              (Transformation|SetWorldLocationAndRotation (Variables|/Game/Blueprints/EndSequence/BP_TarotCard.BP_TarotCard_C|GetDefaultSceneRoot (Variables|Default|GetCard2)) (Transformation|GetWorldLocation _cardlocation2) (Transformation|GetWorldRotation _cardlocation2) false false)
              (elif (Utilities|Name|Equal(Name) _notifyname (Utilities|Name|MakeLiteralName "AddCard3"))
                (bind _returnvalue_5 (Game|SpawnActorfromClass "/Game/Blueprints/EndSequence/BP_TarotCard.BP_TarotCard_C" (Math|Transform|MakeTransform "0, 0, 0" "0, 0,90.000000" "0.500000,0.500000,0.500000") "Undefined" 0 0))
                (bind _output_get_4 (Variables|Default|SetCard3 _returnvalue_5))
                (Transformation|AttachComponentToComponent _output_get_4 (Variables|/Game/Blueprints/BP_PlayedCharacter.BP_PlayedCharacter_C|GetRightArm (Variables|Default|GetPlayedCharacter)) "CardSocket" "KeepRelative" "KeepRelative" "KeepWorld" true)
                (elif (Utilities|Name|Equal(Name) _notifyname (Utilities|Name|MakeLiteralName "ReleaseCard3"))
                  (Transformation|DetachFromActor (Variables|Default|GetCard3) "KeepRelative" "KeepRelative" "KeepRelative")
                  (Transformation|SetWorldScale3D (Variables|/Game/Blueprints/EndSequence/BP_TarotCard.BP_TarotCard_C|GetDefaultSceneRoot (Variables|Default|GetCard3)) "1.000000,1.000000,1.000000")
                  (Transformation|AddActorLocalRotation (Variables|Default|GetCard3) "0.000000,0.000000,-90.000000" false false)
                  (Transformation|SetWorldLocationAndRotation (Variables|/Game/Blueprints/EndSequence/BP_TarotCard.BP_TarotCard_C|GetDefaultSceneRoot (Variables|Default|GetCard3)) (Transformation|GetWorldLocation _cardlocation3) (Transformation|GetWorldRotation _cardlocation3) false false)
                  (elif (Utilities|Name|Equal(Name) _notifyname (Utilities|Name|MakeLiteralName "TakeHammer"))
                    (bind _returnvalue_6 (Game|SpawnActorfromClass "/Game/Blueprints/EndSequence/BP_Hammer.BP_Hammer_C" (Math|Transform|MakeTransform "0, 0, 0" "0, 0,90.000000" "0.500000,0.500000,0.500000") "Undefined" 0 0))
                    (bind _output_get_5 (Variables|Default|SetHammer _returnvalue_6))
                    (Transformation|AttachComponentToComponent _output_get_5 (Variables|/Game/Blueprints/BP_PlayedCharacter.BP_PlayedCharacter_C|GetRightArm (Variables|Default|GetPlayedCharacter)) "HammerSocket" "KeepRelative" "KeepRelative" "KeepWorld" true)))))))))))

(event Custom|MoveNail
  (bind _nail (Variables|Default|GetNail))
  (Audio|PlaySoundatLocation "/Game/Audio/A_NailSplash.A_NailSplash" (Transformation|GetActorLocation) "0, 0, 0" 1.0 1.0 0.0 0 0 0)
  (bind _alpha (Timeline|MovingNail Play)
    (:Update
      (Transformation|SetActorLocation _nail (Math|Vector|Lerp(Vector) (Transformation|GetActorLocation (Variables|Default|GetNail)) (Transformation|GetWorldLocation (Variables|Default|GetNailLocation)) _alpha) false false)
      (Transformation|SetActorScale3D _nail (Math|Vector|Lerp(Vector) (Transformation|GetActorScale3D (Variables|Default|GetNail)) "1.000000,1.000000,1.000000" _alpha)))))

(event Custom|UseTarot
  (bind _mainplayercontroller (CallFunction|GetMainPlayerController))
  (bind _playerlocationtarget (Variables|Default|GetPlayerLocationTarget))
  (bind _playedcharacter (Variables|Default|GetPlayedCharacter))
  (bind _returnvalue (Transformation|GetActorLocation _playedcharacter))
  (bind _returnvalue_2 (Transformation|GetWorldLocation _playerlocationtarget))
  (Widget|RemovefromParent (Variables|Default|GetEndChoice))
  (Actor|Tick|SetActorTickEnabled false)
  (Variables|/Script/Engine.PlayerController|SetbShowMouseCursor _mainplayercontroller true)
  (Input|SetInputModeGameOnly _mainplayercontroller)
  (bind _alpha (Timeline|MoveTowards PlayFromStart)
    (:Update
      (Transformation|SetActorLocation (Variables|Default|GetPlayedCharacter) (Math|Vector|Lerp(Vector) _returnvalue _returnvalue_2 _alpha) false false)
      (if (< (Math|Vector|Distance(Vector) _returnvalue _returnvalue_2) 0.001)
        (Audio|Components|Audio|Stop (Variables|Default|GetMoveTowards))
        (Variables|Default|SetBaseRotation (Pawn|GetControlRotation (CallFunction|GetMainPlayerController) :!class /Script/Engine.Controller))
        (Utilities|FlowControl|DoOnce false
          (:Completed
            (CallFunction|MainAnim)))))))

(event Custom|PickUp
  (bind _mainplayercontroller (CallFunction|GetMainPlayerController))
  (Widget|RemovefromParent (Variables|Default|GetEndChoice))
  (Variables|/Script/Engine.PlayerController|SetbShowMouseCursor _mainplayercontroller true)
  (Input|SetInputModeGameOnly _mainplayercontroller)
  (Actor|Tick|SetActorTickEnabled false)
  (Default|PlayPhoneAnimation (CallFunction|GetMainPlayerController))
  (Audio|PlaySound2D "/Game/Audio/Dialogs/Dialogue_Bad_End.Dialogue_Bad_End" 1.0 1.0 0.0 0 0)
  (Utilities|FlowControl|Delay 32.0)
  (Game|QuitGame 0 "Quit" false))

(event Custom|Bzzz
  (Utilities|FlowControl|DoOnce false :!label _label
    (:Completed
      (Audio|PlaySound2D "/Game/Audio/Phone/A_Phone_Shaking.A_Phone_Shaking" 1.0 1.0 0.0 0 0)
      (Utilities|FlowControl|Delay 2.0)
      (goto _label Reset))))

(event EventBeginPlay
  (bind _returnvalue (UserInterface|CreateWidget "/Game/Blueprints/UI/WBP_EndChoice.WBP_EndChoice_C"))
  (bind _output_get (Variables|Default|SetEndChoice _returnvalue))
  (Variables|/Game/Blueprints/UI/WBP_EndChoice.WBP_EndChoice_C|SetEvent _output_get self))

(event EventThisEventBehavior
  (params (OtherComp :type Primitive%20Component%20Object%20Reference))
  (bind _mainplayercontroller (CallFunction|GetMainPlayerController))
  (bind _asbp_played_character (Utilities|Casting|CastToBP_PlayedCharacter (Components|GetOwner OtherComp)))
  (Variables|Default|SetPlayedCharacter _asbp_played_character)
  (Variables|Default|SetisActive false)
  (Default|EnterCinematicMode (CallFunction|GetMainPlayerController))
  (Variables|Default|SetBaseRotation (Pawn|GetControlRotation (CallFunction|GetMainPlayerController) :!class /Script/Engine.Controller))
  (Physics|SetEnableGravity (Variables|/Script/Engine.Character|GetCapsuleComponent (Variables|Default|GetPlayedCharacter)) false)
  (Collision|SetCollisionEnabled (Variables|/Script/Engine.Character|GetCapsuleComponent (Variables|Default|GetPlayedCharacter)) "NoCollision")
  (Default|DisableHeadBob (Variables|Default|GetPlayedCharacter))
  (bind _rotation (Timeline|FirstLookAtCorpse PlayFromStart)
    (:Update
      (Pawn|SetControlRotation (CallFunction|GetMainPlayerController) (Math|Rotator|Lerp(Rotator) (Variables|Default|GetBaseRotation) (Math|Rotator|FindLookatRotation (Transformation|GetWorldLocation (Variables|/Game/Blueprints/BP_PlayedCharacter.BP_PlayedCharacter_C|GetFirstPersonCamera (Variables|Default|GetPlayedCharacter))) (Transformation|GetWorldLocation (Variables|Default|GetPlayerRotationTarget))) _rotation true))
      (if (Math|Rotator|Equal(Rotator) (Pawn|GetControlRotation (CallFunction|GetMainPlayerController) :!class /Script/Engine.Controller) (Math|Rotator|FindLookatRotation (Transformation|GetWorldLocation (Variables|/Game/Blueprints/BP_PlayedCharacter.BP_PlayedCharacter_C|GetFirstPersonCamera (Variables|Default|GetPlayedCharacter))) (Transformation|GetWorldLocation (Variables|Default|GetPlayerRotationTarget))) 0.0001)
        (Audio|Components|Audio|Stop (Variables|Default|GetFirstLookAtCorpse))
        (Actor|Tick|SetActorTickEnabled true)
        (if (>= (Variables|/Game/Blueprints/BP_MainPlayerController.BP_MainPlayerController_C|GetEssentialItems (CallFunction|GetMainPlayerController)) 2)
          (UserInterface|Viewport|AddtoViewport (Variables|Default|GetEndChoice) 0)
          (Variables|/Script/Engine.PlayerController|SetbShowMouseCursor _mainplayercontroller true)
          (Input|SetInputModeUIOnly _mainplayercontroller 0 "DoNotLock")
          (else
            (Utilities|FlowControl|Delay 5.0)
            (CallFunction|PickUp)))))))

(event EventTick
  (params (DeltaSeconds :type Float%20%28single-precision%29))
  (CallFunction|Bzzz))

(fn ConstructionScript)
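; End-sequence event that plays a scripted first-person cinematic in which the player strikes an approaching Frank with a hammer.
; ThisEventBehavior spawns Frank with AIMoveTo toward the player, then chained timelines move the player and turn the view to Frank, the hammer and Frank's face.
; Tick then watches for Frank to come close and triggers PlayHammerHit.
; The hit montage ends in a fade that removes Frank, activates NextEvent and exits cinematic mode.
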(event Custom|PlayHammerHit
  (bind _nextevent (Variables|Default|GetNextEvent))
  (bind _frank (Variables|Default|GetFrank))
  (Actor|Tick|SetActorTickEnabled false)
  (Actor|DestroyActor (Variables|Default|GetHammer))
  (bind _returnvalue (Game|SpawnActorfromClass "/Game/Blueprints/EndSequence/BP_Hammer.BP_Hammer_C" (Math|Transform|MakeTransform "0, 0, 0" "0, 0,90.000000" "0.500000,0.500000,0.500000") "Undefined" 0 0))
  (bind _output_get (Variables|Default|SetHammer _returnvalue))
  (Transformation|AttachComponentToComponent _output_get (Variables|/Game/Blueprints/BP_PlayedCharacter.BP_PlayedCharacter_C|GetRightArm (Variables|Default|GetPlayedCharacter)) "HammerSocket" "KeepRelative" "KeepRelative" "KeepWorld" true)
  (Default|SetArmsVisibility (Variables|Default|GetPlayedCharacter) true)
  (Components|Animation|SetAnimation (Variables|/Game/Blueprints/BP_PlayedCharacter.BP_PlayedCharacter_C|GetRightArm (Variables|Default|GetPlayedCharacter)) "/Game/Animations/Player/A_HammerHit.A_HammerHit")
  (Animation|Montage|PlayMontage (Variables|/Game/Blueprints/BP_PlayedCharacter.BP_PlayedCharacter_C|GetRightArm (Variables|Default|GetPlayedCharacter)) "/Game/Animations/Player/AM_HammerHit.AM_HammerHit"
    (:OnCompleted
      (Default|SetArmsVisibility (Variables|Default|GetPlayedCharacter) false)
      (Actor|DestroyActor (Variables|Default|GetHammer))
      (CameraFades|StartCameraFade :self (Variables|/Script/Engine.PlayerController|GetPlayerCameraManager (CallFunction|GetMainPlayerController)) :ToAlpha 1.0 :Duration 0.1 :bHoldWhenFinished true)
      (Variables|/Game/Blueprints/Event/BP_EventDaddy.BP_EventDaddy_C|SetisActive _nextevent true)
      (Rendering|SetVisibility (Variables|/Game/Blueprints/EndSequence/BP_RitualScene.BP_RitualScene_C|GetSkeletalMesh _nextevent) true false)
      (Utilities|FlowControl|DoOnce false
        (:Completed
          (Actor|DestroyActor (Variables|/Game/Blueprints/BP_Frank.BP_Frank_C|GetShovel _frank))
          (Actor|DestroyActor _frank)
          (Utilities|FlowControl|Delay 2.0)
          (CameraFades|StartCameraFade :self (Variables|/Script/Engine.PlayerController|GetPlayerCameraManager (CallFunction|GetMainPlayerController)) :FromAlpha 1.0 :Duration 2.0 :bHoldWhenFinished true)
          (Default|ExitCinematicMode (CallFunction|GetMainPlayerController)))))))

(event EventTick
  (params (DeltaSeconds :type Float%20%28single-precision%29))
  (if (< (Transformation|GetDistanceTo (Variables|Default|GetFrank) (Variables|Default|GetPlayedCharacter)) 3e+02)
    (Utilities|FlowControl|DoOnce false
      (:Completed
        (CallFunction|PlayHammerHit)))))

(event EventThisEventBehavior
  (params (OtherComp :type Primitive%20Component%20Object%20Reference))
  (bind _mainplayercontroller (CallFunction|GetMainPlayerController))
  (bind _playermovinglocation (Variables|Default|GetPlayerMovingLocation))
  (bind _rootcomponent (Variables|/Script/Engine.Actor|GetRootComponent _playermovinglocation))
  (bind _returnvalue (Transformation|GetWorldLocation _rootcomponent))
  (bind _asbp_played_character (Utilities|Casting|CastToBP_PlayedCharacter (Components|GetOwner OtherComp)))
  (Variables|Default|SetPlayedCharacter _asbp_played_character)
  (Variables|Default|SetisActive false)
  (Utilities|FlowControl|DoOnce false
    (:Completed
      (Default|EnterCinematicMode (CallFunction|GetMainPlayerController))
      (Utilities|FlowControl|DoOnce false
        (:Completed
          (bind _returnvalue_2 (Game|SpawnActorfromClass "/Game/Blueprints/BP_Frank.BP_Frank_C" (Math|Transform|MakeTransform (Transformation|GetActorLocation (Variables|Default|GetFrankBeginningLocation))) "Undefined" 0 0))
          (bind _output_get (Variables|Default|SetFrank _returnvalue_2))
          (AI|AIMoveTo _output_get "0, 0, 0" (Variables|Default|GetPlayedCharacter) 5.0 false
            (:then
              (Utilities|FlowControl|Delay 2.0)
              (Variables|Default|SetBaseRotation (Pawn|GetControlRotation _mainplayercontroller :!class /Script/Engine.Controller))
              (bind _rotation (Timeline|LookAtFrank PlayFromStart)
                (:Update
                  (Pawn|SetControlRotation _mainplayercontroller (Math|Rotator|Lerp(Rotator) (Variables|Default|GetBaseRotation) (Math|Rotator|FindLookatRotation (Transformation|GetWorldLocation (Variables|/Game/Blueprints/BP_PlayedCharacter.BP_PlayedCharacter_C|GetFirstPersonCamera (Variables|Default|GetPlayedCharacter))) (Transformation|GetActorLocation (Variables|Default|GetFrank))) _rotation true))
                  (if (Math|Rotator|Equal(Rotator) (Pawn|GetControlRotation (CallFunction|GetMainPlayerController) :!class /Script/Engine.Controller) (Math|Rotator|FindLookatRotation (Transformation|GetWorldLocation (Variables|/Game/Blueprints/BP_PlayedCharacter.BP_PlayedCharacter_C|GetFirstPersonCamera (Variables|Default|GetPlayedCharacter))) (Transformation|GetActorLocation (Variables|Default|GetFrank))) 0.0001)
                    (Audio|Components|Audio|Stop (Variables|Default|GetLookAtFrank))
                    (Utilities|FlowControl|Delay 0.8)
                    (Variables|Default|SetBaseRotation (Pawn|GetControlRotation (CallFunction|GetMainPlayerController) :!class /Script/Engine.Controller))
                    (bind _alpha (Timeline|MoveTowards PlayFromStart)
                      (:Update
                        (Transformation|SetActorLocation (Variables|Default|GetPlayedCharacter) (Math|Vector|Lerp(Vector) (Transformation|GetActorLocation (Variables|Default|GetPlayedCharacter)) _returnvalue _alpha) false false)
                        (if (< (Math|Vector|Distance(Vector) (Transformation|GetActorLocation (Variables|Default|GetPlayedCharacter)) _returnvalue) 1e+02)
                          (Audio|Components|Audio|Stop (Variables|Default|GetMoveTowards))
                          (Variables|Default|SetBaseRotation (Pawn|GetControlRotation (CallFunction|GetMainPlayerController) :!class /Script/Engine.Controller))
                          (bind _rotation_2 (Timeline|SecondLookAt PlayFromStart)
                            (:Update
                              (Pawn|SetControlRotation (CallFunction|GetMainPlayerController) (Math|Rotator|Lerp(Rotator) (Variables|Default|GetBaseRotation) (Math|Rotator|FindLookatRotation (Transformation|GetWorldLocation (Variables|/Game/Blueprints/BP_PlayedCharacter.BP_PlayedCharacter_C|GetFirstPersonCamera (Variables|Default|GetPlayedCharacter))) (Transformation|GetWorldLocation (Variables|/Game/Blueprints/BP_Frank.BP_Frank_C|GetFaceLocation (Variables|Default|GetFrank)))) _rotation_2 true))
                              (if (Math|Rotator|Equal(Rotator) (Pawn|GetControlRotation (CallFunction|GetMainPlayerController) :!class /Script/Engine.Controller) (Math|Rotator|FindLookatRotation (Transformation|GetWorldLocation (Variables|/Game/Blueprints/BP_PlayedCharacter.BP_PlayedCharacter_C|GetFirstPersonCamera (Variables|Default|GetPlayedCharacter))) (Transformation|GetWorldLocation (Variables|/Game/Blueprints/BP_Frank.BP_Frank_C|GetFaceLocation (Variables|Default|GetFrank)))) 0.0001)
                                (Audio|Components|Audio|Stop (Variables|Default|GetLookAt))
                                (Utilities|FlowControl|DoOnce false
                                  (:Completed
                                    (Actor|Tick|SetActorTickEnabled true))))))
                          (else
                            (Utilities|FlowControl|DoOnce false
                              (:Completed
                                (bind _rotation_3 (Timeline|LookAt PlayFromStart)
                                  (:Update
                                    (Pawn|SetControlRotation (CallFunction|GetMainPlayerController) (Math|Rotator|Lerp(Rotator) (Variables|Default|GetBaseRotation) (Math|Rotator|FindLookatRotation (Transformation|GetWorldLocation (Variables|/Game/Blueprints/BP_PlayedCharacter.BP_PlayedCharacter_C|GetFirstPersonCamera (Variables|Default|GetPlayedCharacter))) (Transformation|GetActorLocation (Variables|Default|GetHammer))) _rotation_3 true))
                                    (if (Math|Rotator|Equal(Rotator) (Pawn|GetControlRotation (CallFunction|GetMainPlayerController) :!class /Script/Engine.Controller) (Math|Rotator|FindLookatRotation (Transformation|GetWorldLocation (Variables|/Game/Blueprints/BP_PlayedCharacter.BP_PlayedCharacter_C|GetFirstPersonCamera (Variables|Default|GetPlayedCharacter))) (Transformation|GetActorLocation (Variables|Default|GetHammer))) 0.0001)
                                      (Audio|Components|Audio|Stop (Variables|Default|GetLookAt)))))))))))))))))))))

(fn ConstructionScript
  (|CallParentFunction))
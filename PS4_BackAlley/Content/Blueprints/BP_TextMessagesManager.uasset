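; BP_TextMessagesManager is an actor that plays a scripted text conversation with a single sender to the player.
; On BeginPlay it filters DT_TextMessages rows by contact name into parallel arrays of text and sent-by-self flags, then triggers messages on hardcoded delays.
; SendNextMessage advances the index, spawns a BP_TextMessage actor with that content and sender flag, and passes it to the main player controller for adding.
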(event Custom|SendNextMessage
  (bind _sender1index (Variables|Default|GetSender1Index))
  (if (< (Variables|Default|GetSender1Index) (Utilities|Array|Length (Variables|Default|GetSender1Messages)))
    (Math|Integer|IncrementInt (Variables|Default|GetSender1Index)
      (:%20%20
        (bind _returnvalue (Game|SpawnActorfromClass "/Game/Blueprints/BP_TextMessage.BP_TextMessage_C" (Math|Transform|MakeTransform "0, 0, 0") "Undefined" 0 0))
        (Variables|/Game/Blueprints/BP_TextMessage.BP_TextMessage_C|SetSentFromSelf _returnvalue (Utilities|Array|Get(acopy) (Variables|Default|GetSender1SentFromSelf) _sender1index))
        (Variables|/Game/Blueprints/BP_TextMessage.BP_TextMessage_C|SetContent _returnvalue (Utilities|Array|Get(acopy) (Variables|Default|GetSender1Messages) _sender1index))
        (Default|AddNewTextMessage (CallFunction|GetMainPlayerController) _returnvalue)))))

(event EventBeginPlay
  (bind _outrownames (DataTable|GetDataTableRowNames "/Game/Data/DT_TextMessages.DT_TextMessages"))
  (for _array_element _outrownames
    (bind _returnvalue (Utilities|GetDataTableRow "/Game/Data/DT_TextMessages.DT_TextMessages" _array_element)
      (:then
        (if (Utilities|Enum|Equal(Enum) (.Contact (Utilities|Struct|BreakF_TextMessagesStruct _returnvalue)) (Variables|Default|GetSender1Name))
          (Utilities|Array|Add (Variables|Default|GetSender1Messages) (.TextContent (Utilities|Struct|BreakF_TextMessagesStruct _returnvalue)))
          (Utilities|Array|Add (Variables|Default|GetSender1SentFromSelf) (.SentBySelf (Utilities|Struct|BreakF_TextMessagesStruct _returnvalue)))))))
  (Utilities|FlowControl|Delay 2.0)
  (CallFunction|SendNextMessage)
  (Utilities|FlowControl|Delay 2.0)
  (CallFunction|SendNextMessage)
  (Utilities|FlowControl|Delay 1.0)
  (CallFunction|SendNextMessage)
  (Utilities|FlowControl|Delay 1.0)
  (CallFunction|SendNextMessage)
  (Utilities|FlowControl|Delay 1.0)
  (CallFunction|SendNextMessage)
  (Utilities|FlowControl|Delay 1.0)
  (CallFunction|SendNextMessage))

(fn ConstructionScript)
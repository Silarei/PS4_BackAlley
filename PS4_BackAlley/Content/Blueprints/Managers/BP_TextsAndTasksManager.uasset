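; Manager actor that feeds Frank's scripted phone text conversation to the player.
; On BeginPlay it reads DT_TextMessages, keeping contact-filtered message text and sent-by-self flags in parallel arrays.
; It then sends six messages on hard-coded delays, each spawned as a BP_TextMessage actor and passed to the main player controller.
; Despite the name, it contains no task logic.
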(event Custom|SendNextFrankMessage
  (bind _frankmessagesindex (Variables|Default|GetFrankMessagesIndex))
  (if (< (Variables|Default|GetFrankMessagesIndex) (Utilities|Array|Length (Variables|Default|GetFrankMessages)))
    (Math|Integer|IncrementInt (Variables|Default|GetFrankMessagesIndex)
      (:%20%20
        (bind _returnvalue (Game|SpawnActorfromClass "/Game/Blueprints/Managers/BP_TextMessage.BP_TextMessage_C" (Math|Transform|MakeTransform "0, 0, 0") "Undefined" 0 0))
        (Variables|/Game/Blueprints/Managers/BP_TextMessage.BP_TextMessage_C|SetSentFromSelf _returnvalue (Utilities|Array|Get(acopy) (Variables|Default|GetFrankSentFromSelf) _frankmessagesindex))
        (Variables|/Game/Blueprints/Managers/BP_TextMessage.BP_TextMessage_C|SetContent _returnvalue (Utilities|Array|Get(acopy) (Variables|Default|GetFrankMessages) _frankmessagesindex))
        (Default|AddNewTextMessage (CallFunction|GetMainPlayerController) _returnvalue)))))

(event EventBeginPlay
  (|GetFrankMessages))

(fn ConstructionScript)
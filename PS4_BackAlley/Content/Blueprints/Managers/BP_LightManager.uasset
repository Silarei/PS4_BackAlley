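; BP_LightManager is a manager Blueprint that switches a level's lighting between electricity-on and electricity-off states.
; It holds two light arrays, one for each power state.
; SwitchOnLights and SwitchOffLights toggle light component visibility so that one set shows while the other hides.
; In both events the off-state loop is nested inside the on-state loop, so it repeats per on-state light and never runs if that array is empty.
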(event Custom|SwitchOffLights
  (for _array_element (Variables|Default|GetLightsWhenElectricityOn)
    (Rendering|SetVisibility (Variables|/Script/Engine.Light|GetLightComponent _array_element) false false)
    (for _array_element_2 (Variables|Default|GetLightsWhenElectricityOff)
      (Rendering|SetVisibility (Variables|/Script/Engine.Light|GetLightComponent _array_element_2) true false))))

(event Custom|SwitchOnLights
  (for _array_element (Variables|Default|GetLightsWhenElectricityOn)
    (Rendering|SetVisibility (Variables|/Script/Engine.Light|GetLightComponent _array_element) true false)
    (for _array_element_2 (Variables|Default|GetLightsWhenElectricityOff)
      (Rendering|SetVisibility (Variables|/Script/Engine.Light|GetLightComponent _array_element_2) false false))))

(fn ConstructionScript)
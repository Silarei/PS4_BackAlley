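; An interactable door the player can knock on to advance a linked event to its second phase.
; Its AdditionalInteraction function passes through a DoOnce and a knocked-on flag, then checks that the player's capsule overlaps the event's KnockingDetector.
; On success it sets the flag, has the player controller play a knocking animation and disable movement, then calls Phase2 on the event.
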(event EventBeginPlay)

(event Collision|EventActorBeginOverlap
  (params (OtherActor :type Actor%20Object%20Reference)))

(event EventTick
  (params (DeltaSeconds :type Float%20%28single-precision%29))
  (Utilities|FlowControl|Delay 0.2))

(fn ConstructionScript
  (|CallParentFunction))

(fn AdditionalInteraction
  (bind _event (Variables|Default|GetEvent))
  (bind _main_player_controller (Variables|Default|GetMain%20Player%20Controller))
  (Utilities|FlowControl|DoOnce false
    (:Completed
      (if (not (Variables|Default|GetHasBeenKnockedOn))
        (if (Class|PrimitiveComponent|IsOverlappingComponent (Variables|/Script/Engine.Character|GetCapsuleComponent (Game|GetPlayerCharacter 0)) (Variables|/Game/Blueprints/Event/BP_StoryConflict.BP_StoryConflict_C|GetKnockingDetector _event))
          (Variables|Default|SetHasBeenKnockedOn true)
          (Default|PlayTocTocTocAnimation _main_player_controller)
          (Default|DisableMovement _main_player_controller)
          (Default|Phase2 _event _main_player_controller))))))
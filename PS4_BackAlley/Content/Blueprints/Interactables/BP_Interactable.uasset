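; BP_Interactable is a base interactable actor with empty press and release events.
; When selected and not Locked, it binds interact input through the main player controller, registers as the selected interactable and shows its widget.
; The icon is rotated toward the first-person camera once, as it appears.
; Unselection unbinds input, clears the selection, fires the release event and hides the icon.
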(event Custom|SetInteractable
  (params (CurrentlySelected :type BP%20Interactable%20Object%20Reference))
  (Default|SetSelectedInteractable (Variables|Default|GetMain%20Player%20Controller) CurrentlySelected))

(event Custom|InterractPressed)

(event Custom|InterractReleased)

(event Custom|ShowIcon
  (params (widget :type Widget%20Component%20Object%20Reference))
  (Rendering|SetVisibility widget true false)
  (Transformation|SetWorldRotation widget (Math|Rotator|FindLookatRotation (Transformation|GetWorldLocation (Variables|Default|GetInteractionWidget)) (Transformation|GetWorldLocation (Variables|/Game/Blueprints/BP_PlayedCharacter.BP_PlayedCharacter_C|GetFirstPersonCamera (Variables|/Game/Blueprints/BP_MainPlayerController.BP_MainPlayerController_C|GetPlayedCharacter (Variables|Default|GetMain%20Player%20Controller))))) false false))

(event Custom|HideIcon
  (params (widget :type Widget%20Component%20Object%20Reference))
  (Rendering|SetVisibility widget false false))

(event EventBeginPlay
  (Variables|Default|SetMain%20Player%20Controller (CallFunction|GetMainPlayerController)))

(fn ConstructionScript)

(fn OnSelected
  (if (not (Variables|Default|GetLocked))
    (Default|BindOncetoInteract (Variables|Default|GetMain%20Player%20Controller) (EventDispatchers|CreateEvent :!event Custom|InterractPressed) (EventDispatchers|CreateEvent :!event Custom|InterractReleased))
    (CallFunction|SetInteractable self)
    (CallFunction|ShowIcon (Variables|Default|GetInteractionWidget))))

(fn OnUnselected
  (Default|UnbindAllfromInteract (Variables|Default|GetMain%20Player%20Controller))
  (CallFunction|SetInteractable)
  (CallFunction|InterractReleased)
  (CallFunction|HideIcon (Variables|Default|GetInteractionWidget)))
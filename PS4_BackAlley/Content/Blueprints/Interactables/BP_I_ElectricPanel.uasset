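; Interactable electric panel that restores power once its door is open and advances the story.
; Switching back and cutting power both flip breaker buttons and drive the LightsManager and elevator.
; Two flags stage successive restores: client phone call and conflict event, Franck's event, then his chase with flickering lights and a second call.
; Parent Tick pauses while the door is open and power awaits restoring.
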(event Custom|SwitchBackElectricity
  (if (not (Variables|Default|GetSwitchedBack))
    (if (>= (.yaw (Variables|/Script/Engine.SceneComponent|GetRelativeRotation (Variables|Default|GetDoor))) 8e+01)
      (for _array_element (Variables|Default|GetButtons)
        (Transformation|SetRelativeRotation _array_element (Math|Rotator|MakeRotator (* (.Roll (Math|Rotator|BreakRotator (Variables|/Script/Engine.SceneComponent|GetRelativeRotation _array_element))) -1.0) (.Pitch (Math|Rotator|BreakRotator (Variables|/Script/Engine.SceneComponent|GetRelativeRotation _array_element))) (.Yaw (Math|Rotator|BreakRotator (Variables|/Script/Engine.SceneComponent|GetRelativeRotation _array_element)))) false false))
      (Default|SwitchonLights (Variables|Default|GetLightsManager))
      (Audio|PlaySound2D "/Game/Audio/A_disjoncteur_on.A_disjoncteur_on" 1.0 1.0 0.0 0 0)
      (Default|DisableEnable (Variables|Default|GetElevator) true)
      (Variables|Default|SetSwitchedBack true)
      (if (Variables|Default|GetLaunchCallClient)
        (if (Variables|Default|GetLaunchEventFranck)
          (Variables|/Game/Blueprints/Event/BP_EventDaddy.BP_EventDaddy_C|SetisActive (Variables|Default|GetFranckChaseEvent) true)
          (Utilities|FlowControl|Delay 1.5)
          (for _array_element_2 (Variables|/Game/Blueprints/Managers/BP_LightManager.BP_LightManager_C|GetLightsWhenElectricityOn (Variables|Default|GetLightsManager))
            (Variables|/Game/Blueprints/Event/BP_LightCorridor.BP_LightCorridor_C|SetLightIsClicking _array_element_2 true)
            (Default|LightFlickering _array_element_2))
          (Audio|PlaySound2D "/Game/Audio/A_phone_shaking.A_phone_shaking" 1.0 1.0 0.0 0 0 :!label _label)
          (Utilities|FlowControl|Delay 1.2)
          (Variables|Default|SetMyIndex (+ (Variables|Default|GetMyIndex) 1))
          (if (< (Variables|Default|GetMyIndex) 1)
            (goto _label)
            (else
              (Audio|PlaySound2D "/Game/Audio/Dialogue/Dialogue_Second_appel.Dialogue_Second_appel" 1.0 1.0 0.0 0 0 false)))
          (else
            (Default|CompleteTask (Variables|Default|GetTextAndTaskManager) 2)
            (Transformation|SetActorLocationAndRotation (Variables|Default|GetFranck) "-1345.000000,1200.000000, 0")
            (Variables|/Game/Blueprints/Event/BP_EventDaddy.BP_EventDaddy_C|SetisActive (Variables|Default|GetFranckEvent) true)
            (Variables|Default|SetLaunchEventFranck true)))
        (else
          (Variables|Default|SetLaunchCallClient true)
          (Default|CompleteTask (Variables|Default|GetTextAndTaskManager))
          (Utilities|FlowControl|Delay 1e+01)
          (Audio|PlaySound2D "/Game/Audio/A_phone_shaking.A_phone_shaking" 1.0 1.0 0.0 0 0 :!label _label_2)
          (Utilities|FlowControl|Delay 1.2)
          (Variables|Default|SetMyIndex (+ (Variables|Default|GetMyIndex) 1))
          (if (< (Variables|Default|GetMyIndex) 3)
            (goto _label_2)
            (else
              (Audio|PlaySound2D "/Game/Audio/Dialogue/Le_client_se_plaint_du_bruit.Le_client_se_plaint_du_bruit" 1.0 1.0 0.0 0 0 false)
              (Utilities|FlowControl|Delay 12.5)
              (Default|SendNextTask (Variables|Default|GetTextAndTaskManager))
              (Variables|/Game/Blueprints/Event/BP_EventDaddy.BP_EventDaddy_C|SetisActive (Variables|Default|GetEventStoryConflict) true))))))))

(event Custom|CutElectricity
  (for _array_element (Variables|Default|GetButtons)
    (Transformation|SetRelativeRotation _array_element (Math|Rotator|MakeRotator (* (.Roll (Math|Rotator|BreakRotator (Variables|/Script/Engine.SceneComponent|GetRelativeRotation _array_element))) -1.0) (.Pitch (Math|Rotator|BreakRotator (Variables|/Script/Engine.SceneComponent|GetRelativeRotation _array_element))) (.Yaw (Math|Rotator|BreakRotator (Variables|/Script/Engine.SceneComponent|GetRelativeRotation _array_element)))) false false))
  (Default|SwitchOffLights (Variables|Default|GetLightsManager))
  (Variables|Default|SetSwitchedBack false)
  (Default|DisableEnable (Variables|Default|GetElevator) false))

(event EventBeginPlay
  (|CallParentFunction)
  (Utilities|Array|Add (Variables|Default|GetButtons) (Variables|Default|GetButtons1))
  (Utilities|Array|Add (Variables|Default|GetButtons) (Variables|Default|GetButtons2))
  (Utilities|Array|Add (Variables|Default|GetButtons) (Variables|Default|GetButtons4))
  (Utilities|Array|Add (Variables|Default|GetButtons) (Variables|Default|GetButtons5)))

(event EventTick
  (params (DeltaSeconds :type Float%20%28single-precision%29))
  (if (and (<= (.yaw (Variables|/Script/Engine.SceneComponent|GetRelativeRotation (Variables|Default|GetDoor))) 8e+01) (not (Variables|Default|GetSwitchedBack)))
    (|CallParentFunction DeltaSeconds :!label _label)
    (elif (Variables|Default|GetSwitchedBack)
      (goto _label))))

(fn ConstructionScript
  (|CallParentFunction))

(fn AdditionalInteraction
  (CallFunction|SwitchBackElectricity))
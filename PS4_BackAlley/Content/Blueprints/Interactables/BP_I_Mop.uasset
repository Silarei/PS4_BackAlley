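; Pickable mop interactable that the player carries and pushes back and forth to mop.
; The first press attaches it to the played character's capsule, stores its resting pose and disables object selection.
; Later presses lower and tilt the mesh, and releasing restores the stored pose.
; While held, Tick slides the mesh along the character's forward vector using UpRate and sensitivity, replaying the mop sound through a delayed DoOnce throttle.
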(event Custom|Sweep
  (bind _playedcharacter (CallFunction|GetPlayedCharacter))
  (Transformation|SetWorldLocation (Variables|Default|GetStaticMesh) (+ (Transformation|GetWorldLocation (Variables|Default|GetStaticMesh)) (* (Transformation|GetActorForwardVector _playedcharacter) (* (* (Variables|/Game/Blueprints/BP_PlayedCharacter.BP_PlayedCharacter_C|GetUpRate _playedcharacter) (Variables|Default|GetSensitivity)) -1.0))) false false)
  (Utilities|FlowControl|DoOnce false :!label _label
    (:Completed
      (Audio|Components|Audio|Play (Variables|Default|GetMopSound) 0.0)
      (Utilities|FlowControl|Delay 0.5)
      (goto _label Reset))))

(event EventBeginPlay
  (|CallParentFunction) ; This node is disabled and will not be called.\nDrag off pins to build functionality.
)

(event EventInterractReleased
  (bind _staticmesh (Variables|Default|GetStaticMesh))
  (Variables|Default|SetLMBPressed false)
  (Transformation|SetRelativeLocation _staticmesh (Variables|Default|GetOriginalLocation) false false)
  (Transformation|SetRelativeRotation _staticmesh (Variables|Default|GetOriginalRotation) false false))

(event EventTick
  (params (DeltaSeconds :type Float%20%28single-precision%29))
  (if (Variables|Default|GetLMBPressed)
    (CallFunction|Sweep)))

(event EventInterractPressed
  (bind _staticmesh (Variables|Default|GetStaticMesh))
  (bind _staticmesh_2 (Variables|Default|GetStaticMesh))
  (if (Variables|Default|GetIsPicked)
    (Variables|Default|SetLMBPressed true)
    (Transformation|AddRelativeLocation _staticmesh_2 (Math|Vector|MakeVector 2e+01 0.0 -9e+01) false false)
    (Transformation|SetRelativeRotation _staticmesh_2 (Math|Rotator|MakeRotator 45.0 0.0 9e+01) false false)
    (else
      (Transformation|AttachComponentToComponent (Variables|/Script/Engine.Character|GetCapsuleComponent (Variables|/Game/Blueprints/BP_MainPlayerController.BP_MainPlayerController_C|GetPlayedCharacter (Variables|Default|GetMain%20Player%20Controller))) "" "SnapToTarget" "SnapToTarget" "KeepRelative" false)
      (Transformation|AddRelativeLocation _staticmesh (Math|Vector|MakeVector 2e+01 5e+01 8e+01) false false)
      (Transformation|SetRelativeRotation _staticmesh (Math|Rotator|MakeRotator 1e+01 0.0 9e+01) false false)
      (Variables|Default|SetOriginalLocation (Variables|/Script/Engine.SceneComponent|GetRelativeLocation _staticmesh))
      (Variables|Default|SetOriginalRotation (Variables|/Script/Engine.SceneComponent|GetRelativeRotation _staticmesh))
      (Variables|Default|SetIsPicked true)
      (Variables|/Game/Blueprints/BP_MainPlayerController.BP_MainPlayerController_C|SetCanSelectObjects (Variables|Default|GetMain%20Player%20Controller) false))))

(fn ConstructionScript
  (|CallParentFunction))
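; Elevator actor that carries its cabin between placed floor markers, with two sliding doors, sounds and a toggle that enables or disables travel.
; On BeginPlay it links itself to child-actor floor and close buttons, then runs the door toggle.
; Travel requires DoorOpened to be false and lerps the cabin on a timeline whose rate scales with floor distance.
; On arrival it dings and toggles the doors; SetFloor snaps the cabin directly.
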(event Custom|MoveToFloor
  (params (FloorNumber :type Integer))
  (bind _floors (Variables|Default|GetFloors))
  (bind _output (Utilities|Array|Get(acopy) _floors FloorNumber))
  (bind _returnvalue (Transformation|GetActorLocation _output))
  (if (Variables|Default|GetUsable)
    (if (not (Variables|Default|GetDoorOpened))
      (Components|Timeline|SetPlayRate (Variables|Default|GetMovingTimeline) (Math|Float|Absolute(Float) (/ 1.0 (Math|Conversions|ToFloat(Integer) (- FloorNumber (Variables|Default|GetCurrentFloor))))))
      (Audio|Components|Audio|Play (Variables|Default|GetElevatorMoving) 0.0)
      (bind _lerpposition (Timeline|MovingTimeline PlayFromStart)
        (:Update
          (Transformation|SetWorldLocation (Variables|Default|GetElevatorBox) (Math|Vector|Lerp(Vector) (Transformation|GetActorLocation (Utilities|Array|Get(acopy) (Variables|Default|GetFloors) (Variables|Default|GetCurrentFloor))) _returnvalue _lerpposition) false true)
          (if (<= (Math|Vector|Distance(Vector) (Transformation|GetWorldLocation (Variables|Default|GetElevatorBox)) _returnvalue) 0.001)
            (Audio|Components|Audio|Stop (Variables|Default|GetMovingTimeline))
            (Audio|Components|Audio|Stop (Variables|Default|GetElevatorMoving))
            (Audio|PlaySoundatLocation "/Game/Audio/A_elevator_diing.A_elevator_diing" (Transformation|GetActorLocation) "0, 0, 0" 1.0 1.0 0.0 0 0 0)
            (Utilities|FlowControl|Delay 0.8)
            (Variables|Default|SetCurrentFloor FloorNumber)
            (CallFunction|OpenCloseDoor)))))))

(event Custom|SetFloor
  (params (Floor :type Integer))
  (Transformation|SetWorldLocation (Variables|Default|GetElevatorBox) (Transformation|GetWorldLocation (Variables|/Script/Engine.TargetPoint|GetSpriteComponent (Utilities|Array|Get(acopy) (Variables|Default|GetFloors) Floor))) false false)
  (Variables|Default|SetCurrentFloor Floor))

(event Custom|OpenCloseDoor
  (bind _elevatordoor2 (Variables|Default|GetElevatorDoor2))
  (bind _elevatordoor1 (Variables|Default|GetElevatorDoor1))
  (bind _relativelocation (Variables|/Script/Engine.SceneComponent|GetRelativeLocation _elevatordoor1))
  (bind _relativelocation_2 (Variables|/Script/Engine.SceneComponent|GetRelativeLocation _elevatordoor2))
  (bind (_x _y _z) (Math|Vector|BreakVector _relativelocation_2))
  (bind (_x_2 _y_2 _z_2) (Math|Vector|BreakVector _relativelocation))
  (Components|Timeline|SetPlayRate (Variables|Default|GetDoorTimeline) 0.1)
  (Audio|Components|Audio|Play (Variables|Default|GetDoorsClosing) 0.0)
  (if (Variables|Default|GetDoorOpened)
    (Variables|Default|SetDoorTargetPosition -85.0)
    (bind _lerpposition (Timeline|DoorTimeline PlayFromStart)
      (:Update
        (Transformation|SetRelativeLocation (Variables|Default|GetElevatorDoor1) (Math|Vector|Lerp(Vector) _relativelocation (Math|Vector|MakeVector (Variables|Default|GetDoorTargetPosition) _y_2 _z_2) _lerpposition) false false)
        (Transformation|SetRelativeLocation (Variables|Default|GetElevatorDoor2) (Math|Vector|Lerp(Vector) _relativelocation_2 (Math|Vector|MakeVector (* (Variables|Default|GetDoorTargetPosition) -1.0) _y _z) _lerpposition) false false)
        (if (< (Math|Vector|Distance(Vector) _relativelocation_2 (Math|Vector|MakeVector (* (Variables|Default|GetDoorTargetPosition) -1.0) _y _z)) 0.001)
          (Audio|Components|Audio|Stop (Variables|Default|GetDoorTimeline))
          (Variables|Default|SetDoorOpened (not (Variables|Default|GetDoorOpened))))))
    (else
      (Variables|Default|SetDoorTargetPosition 0.0)
      (Timeline|DoorTimeline PlayFromStart))))

(event Custom|DisableEnable
  (Variables|Default|SetUsable (not (Variables|Default|GetUsable))))

(event EventBeginPlay
  (bind _asbp_elevator_floor_button (Utilities|Casting|CastToBP_ElevatorFloorButton (Variables|/Script/Engine.ChildActorComponent|GetChildActor (Variables|Default|GetButton0))))
  (Variables|/Game/Blueprints/Interactables/Elevator/BP_ElevatorFloorButton.BP_ElevatorFloorButton_C|SetElevator _asbp_elevator_floor_button self)
  (Variables|/Game/Blueprints/Interactables/Elevator/BP_ElevatorFloorButton.BP_ElevatorFloorButton_C|SetFloor _asbp_elevator_floor_button 0)
  (bind _asbp_elevator_floor_button_2 (Utilities|Casting|CastToBP_ElevatorFloorButton (Variables|/Script/Engine.ChildActorComponent|GetChildActor (Variables|Default|GetButton1))))
  (Variables|/Game/Blueprints/Interactables/Elevator/BP_ElevatorFloorButton.BP_ElevatorFloorButton_C|SetElevator _asbp_elevator_floor_button_2 self)
  (Variables|/Game/Blueprints/Interactables/Elevator/BP_ElevatorFloorButton.BP_ElevatorFloorButton_C|SetFloor _asbp_elevator_floor_button_2 1)
  (bind _asbp_elevator_floor_button_3 (Utilities|Casting|CastToBP_ElevatorFloorButton (Variables|/Script/Engine.ChildActorComponent|GetChildActor (Variables|Default|GetButton2))))
  (Variables|/Game/Blueprints/Interactables/Elevator/BP_ElevatorFloorButton.BP_ElevatorFloorButton_C|SetElevator _asbp_elevator_floor_button_3 self)
  (Variables|/Game/Blueprints/Interactables/Elevator/BP_ElevatorFloorButton.BP_ElevatorFloorButton_C|SetFloor _asbp_elevator_floor_button_3 2)
  (bind _asbp_elevator_close_button (Utilities|Casting|CastToBP_ElevatorCloseButton (Variables|/Script/Engine.ChildActorComponent|GetChildActor (Variables|Default|GetButtonClose))))
  (Variables|/Game/Blueprints/Interactables/Elevator/BP_ElevatorCloseButton.BP_ElevatorCloseButton_C|SetElevator _asbp_elevator_close_button self)
  (CallFunction|OpenCloseDoor))

(fn ConstructionScript)
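; BP_ElevatorOutsideButton is an interactable call button outside an elevator that summons it to the button's floor.
; On interaction, it toggles the referenced elevator's door if open and waits briefly before continuing.
; It then tells the elevator to move to its Floor value and plays a button sound at its own location, so the sound is also delayed when the door was open.
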(event EventBeginPlay
  (|CallParentFunction))

(event EventInterractPressed
  (if (Variables|/Game/Blueprints/Interactables/Elevator/BP_Elevator.BP_Elevator_C|GetDoorOpened (Variables|Default|GetElevator))
    (Default|OpenCloseDoor (Variables|Default|GetElevator))
    (Utilities|FlowControl|Delay 2.0))
  (Default|MovetoFloor (Variables|Default|GetElevator) (Variables|Default|GetFloor))
  (Audio|PlaySoundatLocation "/Game/Audio/A_elevator_button.A_elevator_button" (Transformation|GetActorLocation) "0, 0, 0" 1.0 1.0 0.0 0 0 0))

(fn ConstructionScript
  (|CallParentFunction))
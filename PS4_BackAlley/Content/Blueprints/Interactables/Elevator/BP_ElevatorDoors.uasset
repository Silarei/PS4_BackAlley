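; Elevator actor with two sliding doors and a box that snaps to the marker of a chosen floor.
; The construction script applies CurrentFloor through SetFloor, positioning the box in the editor.
; OpenCloseDoor runs a slowed timeline that lerps both doors from their current positions toward mirrored X targets, stopping and flipping DoorOpened on arrival.
; DisableEnable toggles a Usable flag, which this graph never reads.
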(event Custom|SetFloor
  (params (Floor :type Integer))
  (Transformation|SetWorldLocation (Variables|Default|GetElevatorBox) (Transformation|GetWorldLocation (Variables|/Script/Engine.TargetPoint|GetSpriteComponent (Utilities|Array|Get(acopy) (Variables|Default|GetFloors) Floor))) false false)
  (Variables|Default|SetCurrentFloor Floor))

(event Custom|OpenCloseDoor
  (bind _elevatordoor2 (Variables|Default|GetElevatorDoor2))
  (bind _elevatordoor1 (Variables|Default|GetElevatorDoor1))
  (bind _relativelocation (Variables|/Script/Engine.SceneComponent|GetRelativeLocation _elevatordoor1))
  (bind _relativelocation_2 (Variables|/Script/Engine.SceneComponent|GetRelativeLocation _elevatordoor2))
  (bind (_x _y _z) (Math|Vector|BreakVector _relativelocation_2))
  (bind (_x_2 _y_2 _z_2) (Math|Vector|BreakVector _relativelocation))
  (Components|Timeline|SetPlayRate (Variables|Default|GetDoorTimeline) 0.1)
  (if (Variables|Default|GetDoorOpened)
    (Variables|Default|SetDoorTargetPosition 0.0)
    (bind _lerpposition (Timeline|DoorTimeline PlayFromStart)
      (:Update
        (Transformation|SetRelativeLocation (Variables|Default|GetElevatorDoor1) (Math|Vector|Lerp(Vector) _relativelocation (Math|Vector|MakeVector (Variables|Default|GetDoorTargetPosition) _y_2 _z_2) _lerpposition) false false)
        (Transformation|SetRelativeLocation (Variables|Default|GetElevatorDoor2) (Math|Vector|Lerp(Vector) _relativelocation_2 (Math|Vector|MakeVector (* (Variables|Default|GetDoorTargetPosition) -1.0) _y _z) _lerpposition) false false)
        (if (< (Math|Vector|Distance(Vector) _relativelocation_2 (Math|Vector|MakeVector (* (Variables|Default|GetDoorTargetPosition) -1.0) _y _z)) 0.001)
          (Audio|Components|Audio|Stop (Variables|Default|GetDoorTimeline))
          (Variables|Default|SetDoorOpened (not (Variables|Default|GetDoorOpened))))))
    (else
      (Variables|Default|SetDoorTargetPosition 85.0)
      (Timeline|DoorTimeline PlayFromStart))))

(event Custom|DisableEnable
  (Variables|Default|SetUsable (not (Variables|Default|GetUsable))))

(event EventBeginPlay)

(fn ConstructionScript
  (CallFunction|SetFloor (Variables|Default|GetCurrentFloor)))
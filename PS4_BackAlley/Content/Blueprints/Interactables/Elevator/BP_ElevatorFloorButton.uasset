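; BP_ElevatorFloorButton is an interactable button that sends an elevator to a specific floor.
; On InterractPressed it calls MoveToFloor on its Elevator reference with its Floor value and plays a button sound at its location.
; BeginPlay creates a dynamic M_Button material instance, stores it and applies it to the static mesh, though this Blueprint sets no parameters on it.
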(event EventBeginPlay
  (|CallParentFunction)
  (bind _returnvalue (Rendering|Material|CreateDynamicMaterialInstance "/Game/Materials/M_Button.M_Button" "None" "None" :!class /Script/Engine.KismetMaterialLibrary))
  (bind _output_get (Variables|Default|SetMaterialInstance _returnvalue))
  (Rendering|Material|SetMaterial (Variables|Default|GetStaticMesh) 0 _output_get))

(event EventInterractPressed
  (Default|MovetoFloor (Variables|Default|GetElevator) (Variables|Default|GetFloor))
  (Audio|PlaySoundatLocation "/Game/Audio/A_elevator_button.A_elevator_button" (Transformation|GetActorLocation) "0, 0, 0" 1.0 1.0 0.0 0 0 0))

(fn ConstructionScript
  (|CallParentFunction))
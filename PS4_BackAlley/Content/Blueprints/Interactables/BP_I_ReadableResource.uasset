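; Interactable readable resource that shows its text to the player through a UI when used.
; On BeginPlay it scans the rows of DT_ReadableResourceTexts and caches the Dialog whose ResourceName matches its own.
; On interact press, the player controller plays a take animation and receives the text, then adds the reading UI after a short delay.
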(event EventBeginPlay
  (|CallParentFunction)
  (bind _outrownames (DataTable|GetDataTableRowNames "/Game/Data/DT_ReadableResourceTexts.DT_ReadableResourceTexts"))
  (for _array_element _outrownames
    (bind _returnvalue (Utilities|GetDataTableRow "/Game/Data/DT_ReadableResourceTexts.DT_ReadableResourceTexts" _array_element)
      (:then
        (if (Utilities|Enum|Equal(Enum) (.resourcename _returnvalue) (Variables|Default|GetResourceName))
          (Variables|Default|SetReadableResourceText (.dialog _returnvalue)))))))

(event EventInterractPressed
  (bind _main_player_controller (Variables|Default|GetMain%20Player%20Controller))
  (Default|PlayTakeAnimation (Variables|Default|GetMain%20Player%20Controller))
  (Default|SetReadableResourceText _main_player_controller (Variables|Default|GetReadableResourceText))
  (Utilities|FlowControl|Delay 1.0)
  (Default|AddReadableResourceUI _main_player_controller))

(event EventInterractReleased)

(fn ConstructionScript
  (|CallParentFunction))
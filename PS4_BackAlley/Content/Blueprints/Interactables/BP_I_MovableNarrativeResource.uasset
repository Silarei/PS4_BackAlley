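; Interactable narrative resource that the player can lift to inspect, rotate and pocket, with its mesh taken from a linked data asset.
; Interacting plays a take animation, moves the mesh before the first-person camera, locks movement and binds turn and right-mouse controller events.
; Turn input adds world rotation derived from camera vectors.
; Interacting again restores transform and movement and unbinds input, while pocketing does the same, then destroys the actor.
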(event Custom|ExitTurningMode
  (bind _staticmesh (Variables|Default|GetStaticMesh))
  (bind _main_player_controller (Variables|Default|GetMain%20Player%20Controller))
  (Transformation|SetWorldLocation _staticmesh (Variables|Default|GetOriginalLocation) false false)
  (Transformation|SetRelativeRotation _staticmesh (Variables|Default|GetOriginalRotation) false false)
  (Default|UnbindAllfromTurnObjectRight _main_player_controller)
  (Default|UnbindAllfromTurnObjectUp _main_player_controller)
  (Default|UnbindAllfromRMBPressed _main_player_controller)
  (Default|EnableMovement _main_player_controller))

(event Custom|TurnObjectRight
  (params (Axis%20Value :type Float%20%28single-precision%29))
  (bind _returnvalue (* Axis%20Value -1.0))
  (bind _main_player_controller (Variables|Default|GetMain%20Player%20Controller))
  (bind _playedcharacter (Variables|/Game/Blueprints/BP_MainPlayerController.BP_MainPlayerController_C|GetPlayedCharacter _main_player_controller))
  (bind _firstpersoncamera (Variables|/Game/Blueprints/BP_PlayedCharacter.BP_PlayedCharacter_C|GetFirstPersonCamera _playedcharacter))
  (bind _returnvalue_2 (Math|Vector|GetForwardVector _firstpersoncamera))
  (bind _returnvalue_3 (* _returnvalue_2 _returnvalue))
  (bind (_x _y _z) (Math|Vector|BreakVector _returnvalue_3))
  (Transformation|AddWorldRotation (Variables|Default|GetStaticMesh) (Math|Rotator|MakeRotator _x _y _z) false false))

(event Custom|TurnObjectUp
  (params (Axis%20Value :type Float%20%28single-precision%29))
  (bind _returnvalue (* Axis%20Value -1.0))
  (bind _main_player_controller (Variables|Default|GetMain%20Player%20Controller))
  (bind _playedcharacter (Variables|/Game/Blueprints/BP_MainPlayerController.BP_MainPlayerController_C|GetPlayedCharacter _main_player_controller))
  (bind _firstpersoncamera (Variables|/Game/Blueprints/BP_PlayedCharacter.BP_PlayedCharacter_C|GetFirstPersonCamera _playedcharacter))
  (bind _returnvalue_2 (Math|Vector|GetRightVector _firstpersoncamera))
  (bind _returnvalue_3 (* _returnvalue_2 _returnvalue))
  (bind (_x _y _z) (Math|Vector|BreakVector _returnvalue_3))
  (Transformation|AddWorldRotation (Variables|Default|GetStaticMesh) (Math|Rotator|MakeRotator _x _y _z) false false))

(event Custom|PocketItem
  (CallFunction|ExitTurningMode)
  (Actor|DestroyActor))

(event EventBeginPlay
  (bind _staticmesh (Variables|Default|GetStaticMesh))
  (|CallParentFunction)
  (Variables|Default|SetOriginalLocation (Transformation|GetWorldLocation _staticmesh))
  (Variables|Default|SetOriginalRotation (Variables|/Script/Engine.SceneComponent|GetRelativeRotation _staticmesh)))

(event EventInterractPressed
  (bind _playedcharacter (CallFunction|GetPlayedCharacter))
  (bind _main_player_controller (Variables|Default|GetMain%20Player%20Controller))
  (bind _firstpersoncamera (Variables|/Game/Blueprints/BP_PlayedCharacter.BP_PlayedCharacter_C|GetFirstPersonCamera _playedcharacter))
  (if (Variables|Default|GetIsInMoveMode)
    (Variables|Default|SetIsInMoveMode false)
    (CallFunction|ExitTurningMode)
    (else
      (Variables|Default|SetIsInMoveMode true)
      (Default|PlayTakeAnimation (Variables|Default|GetMain%20Player%20Controller))
      (Utilities|FlowControl|Delay 1.0)
      (Transformation|SetWorldLocation (Variables|Default|GetStaticMesh) (+ (Transformation|GetWorldLocation _firstpersoncamera) (* (Math|Vector|GetForwardVector _firstpersoncamera) (Variables|Default|GetDistanceFromCamera))) false false)
      (Default|DisableMovement _main_player_controller)
      (Default|BindOncetoTurnObjectRight _main_player_controller (EventDispatchers|CreateEvent :!event Custom|TurnObjectRight))
      (Default|BindOncetoTurnObjectUp _main_player_controller (EventDispatchers|CreateEvent :!event Custom|TurnObjectUp))
      (Default|BindOncetoRMBPressed _main_player_controller (EventDispatchers|CreateEvent :!event Custom|PocketItem)))))

(fn ConstructionScript
  (|CallParentFunction)
  (Components|StaticMesh|SetStaticMesh (Variables|Default|GetStaticMesh) (Variables|/Game/Blueprints/PrimaryDataAssets/BP_DA_PickableItem.BP_DA_PickableItem_C|GetStaticMesh (Variables|Default|GetLinkedDataAsset))))
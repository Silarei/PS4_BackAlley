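; Scripted horror-style event, named for room entry, that makes a spirit vanish and leads into a phone call.
; While active, Tick uses a DoOnce to make the spirit appear and start the room light flickering.
; The event behavior hides the spirit, waits, then stops the light clicking once.
; A delayed counter loop repeats the phone vibration sound before playing the first-call dialogue.
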(event EventTick
  (params (DeltaSeconds :type Float%20%28single-precision%29))
  (if (Variables|Default|GetisActive)
    (Utilities|FlowControl|DoOnce false
      (:Completed
        (Default|Appear (Variables|Default|GetSpirit))
        (Default|LightFlickering (Variables|Default|GetLightRoomSpirit))))))

(event EventThisEventBehavior
  (params (OtherComp :type Primitive%20Component%20Object%20Reference))
  (Default|Disappear (Variables|Default|GetSpirit))
  (Utilities|FlowControl|Delay 6.0)
  (Utilities|FlowControl|DoOnce false
    (:Completed
      (Variables|/Game/Blueprints/Event/BP_LightCorridor.BP_LightCorridor_C|SetLightIsClicking (Variables|Default|GetLightRoomSpirit) false)
      (Audio|PlaySound2D "/Game/Audio/A_phone_shaking.A_phone_shaking" 1.0 1.0 0.0 0 0 :!label _label)
      (Utilities|FlowControl|Delay 1.2)
      (Variables|Default|SetMyIndex (+ (Variables|Default|GetMyIndex) 1))
      (if (< (Variables|Default|GetMyIndex) 3)
        (goto _label)
        (else
          (Audio|PlaySound2D "/Game/Audio/Dialogue/Dialogue_Premier_appel.Dialogue_Premier_appel" 1.0 1.0 0.0 0 0))))))

(fn ConstructionScript
  (|CallParentFunction))
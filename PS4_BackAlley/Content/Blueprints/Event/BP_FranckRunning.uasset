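; BP_FranckRunning is a scripted event that sends Frank running at the player.
; When triggered by the played character, it spawns BP_Frank once at FranckBeginningLocation and starts an AI move toward the player.
; It immediately calls Frank's Running function and activates the next event in the chain, then destroys Frank and his shovel after a fixed delay.
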(event EventThisEventBehavior
  (params (OtherComp :type Primitive%20Component%20Object%20Reference))
  (bind _asbp_played_character (Utilities|Casting|CastToBP_PlayedCharacter (Components|GetOwner OtherComp)))
  (Variables|Default|SetPlayedCharacter _asbp_played_character)
  (Utilities|FlowControl|DoOnce false
    (:Completed
      (bind _returnvalue (Game|SpawnActorfromClass "/Game/Blueprints/BP_Frank.BP_Frank_C" (Math|Transform|MakeTransform (Transformation|GetActorLocation (Variables|Default|GetFranckBeginningLocation))) "Undefined" 0 0))
      (bind _output_get (Variables|Default|SetFrank _returnvalue))
      (AI|AIMoveTo _output_get "0, 0, 0" (Variables|Default|GetPlayedCharacter) 5.0 false
        (:then
          (Default|Running _output_get)
          (Variables|/Game/Blueprints/Event/BP_EventDaddy.BP_EventDaddy_C|SetisActive (Variables|Default|GetNextEvent) true)
          (Utilities|FlowControl|Delay 25.0)
          (Actor|DestroyActor (Variables|/Game/Blueprints/BP_Frank.BP_Frank_C|GetShovel (Variables|Default|GetFrank)))
          (Actor|DestroyActor (Variables|Default|GetFrank)))))))

(fn ConstructionScript
  (|CallParentFunction))
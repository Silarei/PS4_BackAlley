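; BP_FranckTalk is a one-shot scripted event that plays a discussion dialogue while the player is held in place.
; When triggered, it disables player movement, and a timeline turns the control rotation toward a fixed yaw, zeroing pitch and roll.
; It then plays the dialogue sound at a hardcoded world location, waits a fixed delay for it to play, restores movement and destroys itself.
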(event EventThisEventBehavior
  (params (OtherComp :type Primitive%20Component%20Object%20Reference))
  (bind _mainplayercontroller (CallFunction|GetMainPlayerController))
  (Utilities|FlowControl|DoOnce false
    (:Completed
      (Default|DisableMovement _mainplayercontroller)
      (bind _rotation (Timeline|RotationTime Play)
        (:Update
          (Pawn|SetControlRotation _mainplayercontroller (Math|Rotator|MakeRotator 0.0 0.0 (.Yaw (Math|Rotator|BreakRotator (Math|Rotator|Lerp(Rotator) (Pawn|GetControlRotation _mainplayercontroller :!class /Script/Engine.Controller) "0,-90.000000, 0" _rotation))))))
        (:Finished
          (Audio|PlaySoundatLocation "/Game/Audio/Dialogue/Dialogue_Discussion.Dialogue_Discussion" "6180.000000,-6400.000000,-80.000000" "0, 0, 0" 1.0 1.0 0.0 0 0 0)
          (Utilities|FlowControl|Delay 36.0)
          (Default|EnableMovement (CallFunction|GetMainPlayerController))
          (Actor|DestroyActor))))))

(fn ConstructionScript
  (|CallParentFunction))
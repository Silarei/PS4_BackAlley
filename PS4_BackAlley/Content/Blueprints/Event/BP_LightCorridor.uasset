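; BP_LightCorridor is a light Blueprint, named for corridors, that makes its point light flicker irregularly.
; The LightFlickering event randomly picks one of four preset timing sets, then toggles the light on and off twice with delays between changes.
; It calls itself again while LightIsClicking is true, re-rolling the timings each cycle; nothing in this Blueprint's graphs starts the event or sets that flag.
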(event Custom|LightFlickering
  (if (Math|Random|RandomBool)
    (if (Math|Random|RandomBool)
      (Variables|Default|SetDuration1 0.2)
      (Variables|Default|SetDuration2 0.1)
      (Variables|Default|SetDuration3 0.3)
      (else
        (Variables|Default|SetDuration1 0.1)
        (Variables|Default|SetDuration2 0.4)
        (Variables|Default|SetDuration3 0.2)))
    (elif (Math|Random|RandomBool)
      (Variables|Default|SetDuration1 0.4)
      (Variables|Default|SetDuration2 0.3)
      (Variables|Default|SetDuration3 0.1)
      (else
        (Variables|Default|SetDuration1 0.3)
        (Variables|Default|SetDuration2 0.2)
        (Variables|Default|SetDuration3 0.4))))
  (Rendering|SetVisibility (Variables|Default|GetPointLightComponent) true false)
  (Utilities|FlowControl|Delay (Variables|Default|GetDuration1))
  (Rendering|SetVisibility (Variables|Default|GetPointLightComponent) false false)
  (Utilities|FlowControl|Delay (Variables|Default|GetDuration2))
  (Rendering|SetVisibility (Variables|Default|GetPointLightComponent) true false)
  (Utilities|FlowControl|Delay (Variables|Default|GetDuration3))
  (Rendering|SetVisibility (Variables|Default|GetPointLightComponent) false false)
  (Utilities|FlowControl|Delay (Variables|Default|GetDuration1))
  (if (Variables|Default|GetLightIsClicking)
    (CallFunction|LightFlickering)))

(fn ConstructionScript)
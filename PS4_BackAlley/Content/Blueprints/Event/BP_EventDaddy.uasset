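; Base Blueprint for player-triggered events, with an empty ThisEventBehavior event as the hook for the actual behavior.
; Collider overlap runs a check that fires the hook when the player pawn overlaps with a component other than its VisionCube and IsActive is set.
; A failed check retries itself every 0.2 seconds with the same arguments while the player stays inside the Collider.
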(event OnComponentBeginOverlap(Collider)
  (params (OverlappedComponent :type Primitive%20Component%20Object%20Reference) (OtherActor :type Actor%20Object%20Reference) (OtherComp :type Primitive%20Component%20Object%20Reference) (OtherBodyIndex :type Integer) (bFromSweep :type Boolean) (SweepResult :type Hit%20Result%20Structure%20%28by%20ref%29))
  (CallFunction|TestBeforeLaunchingBehavior OtherActor OtherComp))

(event Custom|ThisEventBehavior
  (params (OtherComp :type Primitive%20Component%20Object%20Reference)))

(event Custom|TestBeforeLaunchingBehavior
  (params (Other%20Actor :type Actor%20Object%20Reference) (Other%20Comp :type Primitive%20Component%20Object%20Reference))
  (bind _returnvalue (Game|GetPlayerCharacter 0))
  (bind _asbp_played_character (Utilities|Casting|CastToBP_PlayedCharacter _returnvalue))
  (if (== _returnvalue Other%20Actor)
    (if (!= Other%20Comp (Variables|/Game/Blueprints/BP_PlayedCharacter.BP_PlayedCharacter_C|GetVisionCube _asbp_played_character))
      (if (Variables|Default|GetisActive)
        (if (Collision|IsOverlappingActor (Variables|Default|GetCollider) (Game|GetPlayerCharacter 0) :!class /Script/Engine.PrimitiveComponent)
          (CallFunction|ThisEventBehavior Other%20Comp)
          (else
            (if (Collision|IsOverlappingActor (Variables|Default|GetCollider) _returnvalue :!class /Script/Engine.PrimitiveComponent) :!label _label
              (Utilities|FlowControl|Delay 0.2)
              (CallFunction|TestBeforeLaunchingBehavior Other%20Actor Other%20Comp))))
        (else
          (goto _label)))
      (else
        (goto _label)))
    (else
      (goto _label))))

(fn ConstructionScript)
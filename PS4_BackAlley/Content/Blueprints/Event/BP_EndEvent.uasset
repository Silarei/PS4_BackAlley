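; End-of-game event that runs a scripted first-person cinematic when the player character sets it off.
; It enters cinematic mode, spawns Frank at a marker and sends him toward the player with AI movement.
; Chained timelines turn the control rotation toward Frank, glide the player to a marker while re-aiming, then turn to a final target.
; Each stage advances on a rotation or distance check, ending in a hammer-hit arm montage.
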(event Custom|PlayHammerHit
  (Default|SetArmsVisibility (Variables|Default|GetPlayedCharacter) true)
  (Components|Animation|SetAnimation (Variables|/Game/Blueprints/BP_PlayedCharacter.BP_PlayedCharacter_C|GetRightArm (Variables|Default|GetPlayedCharacter)) "/Game/Animations/Test/A_HammerHit.A_HammerHit")
  (Animation|Montage|PlayMontage (Variables|/Game/Blueprints/BP_PlayedCharacter.BP_PlayedCharacter_C|GetRightArm (Variables|Default|GetPlayedCharacter)) "/Game/Animations/Test/AM_HammerHit.AM_HammerHit"
    (:OnCompleted
      (Default|SetArmsVisibility (Variables|Default|GetPlayedCharacter) false))))

(event EventThisEventBehavior
  (params (OtherComp :type Primitive%20Component%20Object%20Reference))
  (bind _mainplayercontroller (CallFunction|GetMainPlayerController))
  (bind _playermovinglocation (Variables|Default|GetPlayerMovingLocation))
  (bind _rootcomponent (Variables|/Script/Engine.Actor|GetRootComponent _playermovinglocation))
  (bind _returnvalue (Transformation|GetWorldLocation _rootcomponent))
  (bind _asbp_played_character (Utilities|Casting|CastToBP_PlayedCharacter (Components|GetOwner OtherComp)))
  (Variables|Default|SetPlayedCharacter _asbp_played_character)
  (Default|EnterCinematicMode (CallFunction|GetMainPlayerController))
  (Utilities|FlowControl|DoOnce false
    (:Completed
      (bind _returnvalue_2 (Game|SpawnActorfromClass "/Game/Blueprints/BP_Frank.BP_Frank_C" (Math|Transform|MakeTransform (Transformation|GetActorLocation (Variables|Default|GetFrankBeginningLocation))) "Undefined" 0 0))
      (bind _output_get (Variables|Default|SetFrank _returnvalue_2))
      (AI|AIMoveTo _output_get "0, 0, 0" (Variables|Default|GetPlayedCharacter) 5.0 false
        (:then
          (Utilities|FlowControl|Delay 2.0)
          (Variables|Default|SetBaseRotation (Pawn|GetControlRotation _mainplayercontroller :!class /Script/Engine.Controller))
          (bind _rotation (Timeline|LookAtFrank PlayFromStart)
            (:Update
              (Pawn|SetControlRotation _mainplayercontroller (Math|Rotator|Lerp(Rotator) (Variables|Default|GetBaseRotation) (Math|Rotator|FindLookatRotation (Transformation|GetWorldLocation (Variables|/Game/Blueprints/BP_PlayedCharacter.BP_PlayedCharacter_C|GetFirstPersonCamera (Variables|Default|GetPlayedCharacter))) (Transformation|GetActorLocation (Variables|Default|GetFrank))) _rotation true))
              (if (Math|Rotator|Equal(Rotator) (Pawn|GetControlRotation (CallFunction|GetMainPlayerController) :!class /Script/Engine.Controller) (Math|Rotator|FindLookatRotation (Transformation|GetWorldLocation (Variables|/Game/Blueprints/BP_PlayedCharacter.BP_PlayedCharacter_C|GetFirstPersonCamera (Variables|Default|GetPlayedCharacter))) (Transformation|GetActorLocation (Variables|Default|GetFrank))) 0.0001)
                (Audio|Components|Audio|Stop (Variables|Default|GetLookAtFrank))
                (Utilities|FlowControl|Delay 0.8)
                (Variables|Default|SetBaseRotation (Pawn|GetControlRotation (CallFunction|GetMainPlayerController) :!class /Script/Engine.Controller))
                (bind _alpha (Timeline|MoveTowards PlayFromStart)
                  (:Update
                    (Transformation|SetActorLocation (Variables|Default|GetPlayedCharacter) (Math|Vector|Lerp(Vector) (Transformation|GetActorLocation (Variables|Default|GetPlayedCharacter)) _returnvalue _alpha) false false)
                    (if (< (Math|Vector|Distance(Vector) (Transformation|GetActorLocation (Variables|Default|GetPlayedCharacter)) _returnvalue) 1e+02)
                      (Development|PrintString "Hello")
                      (Audio|Components|Audio|Stop (Variables|Default|GetMoveTowards))
                      (Variables|Default|SetBaseRotation (Pawn|GetControlRotation (CallFunction|GetMainPlayerController) :!class /Script/Engine.Controller))
                      (bind _rotation_2 (Timeline|SecondLookAt PlayFromStart)
                        (:Update
                          (Pawn|SetControlRotation (CallFunction|GetMainPlayerController) (Math|Rotator|Lerp(Rotator) (Variables|Default|GetBaseRotation) (Math|Rotator|FindLookatRotation (Transformation|GetWorldLocation (Variables|/Game/Blueprints/BP_PlayedCharacter.BP_PlayedCharacter_C|GetFirstPersonCamera (Variables|Default|GetPlayedCharacter))) (Transformation|GetActorLocation (Variables|Default|GetFirstLookAt))) _rotation_2 true))
                          (if (Math|Rotator|Equal(Rotator) (Pawn|GetControlRotation (CallFunction|GetMainPlayerController) :!class /Script/Engine.Controller) (Math|Rotator|FindLookatRotation (Transformation|GetWorldLocation (Variables|/Game/Blueprints/BP_PlayedCharacter.BP_PlayedCharacter_C|GetFirstPersonCamera (Variables|Default|GetPlayedCharacter))) (Transformation|GetActorLocation (Variables|Default|GetFirstLookAt))) 0.0001)
                            (Audio|Components|Audio|Stop (Variables|Default|GetLookAt))
                            (CallFunction|PlayHammerHit))))
                      (else
                        (Utilities|FlowControl|DoOnce false
                          (:Completed
                            (bind _rotation_3 (Timeline|LookAt PlayFromStart)
                              (:Update
                                (Pawn|SetControlRotation (CallFunction|GetMainPlayerController) (Math|Rotator|Lerp(Rotator) (Variables|Default|GetBaseRotation) (Math|Rotator|FindLookatRotation (Transformation|GetWorldLocation (Variables|/Game/Blueprints/BP_PlayedCharacter.BP_PlayedCharacter_C|GetFirstPersonCamera (Variables|Default|GetPlayedCharacter))) (Transformation|GetActorLocation (Variables|Default|GetSecondLookAtLocation))) _rotation_3 true))
                                (if (Math|Rotator|Equal(Rotator) (Pawn|GetControlRotation (CallFunction|GetMainPlayerController) :!class /Script/Engine.Controller) (Math|Rotator|FindLookatRotation (Transformation|GetWorldLocation (Variables|/Game/Blueprints/BP_PlayedCharacter.BP_PlayedCharacter_C|GetFirstPersonCamera (Variables|Default|GetPlayedCharacter))) (Transformation|GetActorLocation (Variables|Default|GetSecondLookAtLocation))) 0.0001)
                                  (Audio|Components|Audio|Stop (Variables|Default|GetLookAt)))))))))))))))))))

(fn ConstructionScript
  (|CallParentFunction))
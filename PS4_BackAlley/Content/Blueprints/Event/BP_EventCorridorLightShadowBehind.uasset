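; Corridor scare event that flickers the lights and brings a spirit shadow onto the player.
; When ThisEventBehavior runs and the breaker (Disjoncteur) is not switched back, it sets every light in ListLights clicking and starts its flicker.
; It then calls Shadow, which teleports the Spirit's cloud and cube components to fixed vertical offsets below and above the player pawn's location.
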(event Custom|Shadow
  (bind _returnvalue (Game|Player|GetPlayerPawn 0))
  (bind _returnvalue_2 (Transformation|GetActorLocation _returnvalue))
  (Transformation|SetWorldLocation (Variables|/Game/VFX/BP_Spirit_001.BP_Spirit_001_C|GetNS%20Cloud%20001 (Variables|Default|GetSpirit)) (+ _returnvalue_2 "0, 0,-90.000000") false false)
  (Transformation|SetWorldLocation (Variables|/Game/VFX/BP_Spirit_001.BP_Spirit_001_C|GetCube (Variables|Default|GetSpirit)) (+ _returnvalue_2 "0, 0,170.000000") false false))

(event EventThisEventBehavior
  (params (OtherComp :type Primitive%20Component%20Object%20Reference))
  (if (not (Variables|/Game/Blueprints/Interactables/BP_I_ElectricPanel.BP_I_ElectricPanel_C|GetSwitchedBack (Variables|Default|GetDisjoncteur)))
    (for _array_element (Variables|Default|GetListLights)
      (Variables|/Game/Blueprints/Event/BP_LightCorridor.BP_LightCorridor_C|SetLightIsClicking _array_element true)
      (Default|LightFlickering _array_element))
    (CallFunction|Shadow)))

(fn ConstructionScript
  (|CallParentFunction))
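; BP_FirstLightOut is a one-shot scripted event that plays the introduction, then triggers the first power cut.
; If active on BeginPlay, it runs a timed Delay chain: cinematic mode with intro dialogue, a camera fade to teleport the player, then control returns.
; It then has Disjoncteur cut electricity, plays a reaction voice line, advances the task via TextAndTaskManager and destroys itself.
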(event EventBeginPlay
  (CallFunction|ThisEventBehavior))

(event EventThisEventBehavior
  (params (OtherComp :type Primitive%20Component%20Object%20Reference))
  (bind _mainplayercontroller (CallFunction|GetMainPlayerController))
  (bind _playercameramanager (Variables|/Script/Engine.PlayerController|GetPlayerCameraManager _mainplayercontroller))
  (if (Variables|Default|GetisActive)
    (Utilities|FlowControl|DoOnce false
      (:Completed
        (Utilities|FlowControl|Delay 0.2)
        (Default|EnterCinematicMode (CallFunction|GetMainPlayerController))
        (Utilities|FlowControl|Delay 1.0)
        (Audio|PlaySound2D "/Game/Audio/Dialogue/Dialogue_Introduction.Dialogue_Introduction" 1.0 1.0 0.0 0 0)
        (Utilities|FlowControl|Delay 28.0)
        (CameraFades|StartCameraFade :self _playercameramanager :ToAlpha 1.0 :Duration 2.0 :bHoldWhenFinished true)
        (Utilities|FlowControl|Delay 3.0)
        (Transformation|SetActorLocationAndRotation (Game|GetPlayerCharacter 0) "-600.000000,-2230.000000,100.000000" "0,-90.000000,0.000000")
        (CameraFades|StartCameraFade :self _playercameramanager :FromAlpha 1.0 :Duration 2.0 :bHoldWhenFinished true)
        (Default|ExitCinematicMode (CallFunction|GetMainPlayerController))
        (Utilities|FlowControl|Delay 5.0)
        (Default|CutElectricity (Variables|Default|GetDisjoncteur))
        (Utilities|FlowControl|Delay 0.5)
        (Audio|PlaySound2D "/Game/Audio/Dialogue/Lucas_Peter_Les_plombs.Lucas_Peter_Les_plombs" 1.0 1.0 0.0 0 0)
        (Utilities|FlowControl|Delay 5.5)
        (Default|SendNextTask (Variables|Default|GetTextAndTaskManager))
        (Actor|DestroyActor)))))

(fn ConstructionScript
  (|CallParentFunction))
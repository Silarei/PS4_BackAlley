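; BP_StoryConflict is a scripted story event in which a spirit appears and the electricity is cut.
; ThisEventBehavior makes the Spirit appear once, guarded by a DoOnce.
; Phase2 completes a task, then after a short delay restores player movement, sends the next task, cuts power through the Disjoncteur (circuit breaker) and activates the next event in the chain.
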(event Custom|Phase2
  (params (PlayerController :type BP%20Main%20Player%20Controller%20Object%20Reference))
  (Default|CompleteTask (Variables|Default|GetTaskAndTextManager))
  (Utilities|FlowControl|Delay 4.67)
  (Default|EnableMovement PlayerController)
  (Default|SendNextTask (Variables|Default|GetTaskAndTextManager))
  (Default|CutElectricity (Variables|Default|GetDisjoncteur))
  (Variables|/Game/Blueprints/Event/BP_EventDaddy.BP_EventDaddy_C|SetisActive (Variables|Default|GetNextEvent) true))

(event EventThisEventBehavior
  (params (OtherComp :type Primitive%20Component%20Object%20Reference))
  (Utilities|FlowControl|DoOnce false
    (:Completed
      (Default|Appear (Variables|Default|GetSpirit)))))

(fn ConstructionScript
  (|CallParentFunction))
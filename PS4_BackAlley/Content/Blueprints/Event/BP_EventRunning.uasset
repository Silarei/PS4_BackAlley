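; BP_EventRunning is a scripted level event that reshapes the environment in two one-shot stages.
; While IsActive, Tick's DoOnce drops the Escaliers (stairs) meshes and shifts Wall1 upward.
; ThisEventBehavior shifts Wall2 upward once, then after a delay plays a timeline that rotates the Door's yaw.
; That timeline update also clears LightIsClicking on the LightManager's electricity-on lights.
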(event Collision|EventActorBeginOverlap
  (params (OtherActor :type Actor%20Object%20Reference)))

(event EventTick
  (params (DeltaSeconds :type Float%20%28single-precision%29))
  (if (Variables|Default|GetisActive)
    (Utilities|FlowControl|DoOnce false
      (:Completed
        (for _array_element (Variables|Default|GetEscaliers)
          (Transformation|AddRelativeLocation (Variables|/Script/Engine.StaticMeshActor|GetStaticMeshComponent _array_element) "0, 0,-401.000000" false false))
        (Transformation|AddRelativeLocation (Variables|/Script/Engine.StaticMeshActor|GetStaticMeshComponent (Variables|Default|GetWall1)) "0, 0,2000.000000" false false)))))

(event EventThisEventBehavior
  (params (OtherComp :type Primitive%20Component%20Object%20Reference))
  (Utilities|FlowControl|DoOnce false
    (:Completed
      (Transformation|AddRelativeLocation (Variables|/Script/Engine.StaticMeshActor|GetStaticMeshComponent (Variables|Default|GetWall2)) "0, 0,2000.000000" false false)
      (Utilities|FlowControl|Delay 3.0)
      (bind _doorrotation (Timeline|Timeline_0 Play)
        (:Update
          (Transformation|SetRelativeRotation (Variables|/Game/Blueprints/Interactables/BP_Door.BP_Door_C|GetDoor (Variables|Default|GetDoor)) (Math|Rotator|MakeRotator 0.0 0.0 _doorrotation) false false)
          (for _array_element (Variables|/Game/Blueprints/Managers/BP_LightManager.BP_LightManager_C|GetLightsWhenElectricityOn (Variables|Default|GetLightManager))
            (Variables|/Game/Blueprints/Event/BP_LightCorridor.BP_LightCorridor_C|SetLightIsClicking _array_element false)))))))

(fn ConstructionScript
  (|CallParentFunction))
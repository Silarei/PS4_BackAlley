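; Scripted event in an event chain, named for a shadow leading to a room, that pairs a flickering light and a spirit with an opening door.
; Once active, Tick uses a DoOnce to start the light flickering a single time.
; ThisEventBehavior clears the light's flicker flag, makes the spirit disappear and swings the door open with a yaw Timeline.
; When the Timeline finishes, it activates NextEvent and destroys itself.
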(event EventTick
  (params (DeltaSeconds :type Float%20%28single-precision%29))
  (bind _light (Variables|Default|GetLight))
  (if (Variables|Default|GetisActive)
    (Utilities|FlowControl|DoOnce false
      (:Completed
        (Variables|/Game/Blueprints/Event/BP_LightCorridor.BP_LightCorridor_C|SetLightIsClicking _light true)
        (Default|LightFlickering _light)))))

(event EventThisEventBehavior
  (params (OtherComp :type Primitive%20Component%20Object%20Reference))
  (Variables|/Game/Blueprints/Event/BP_LightCorridor.BP_LightCorridor_C|SetLightIsClicking (Variables|Default|GetLight) false)
  (Default|Disappear (Variables|Default|GetSpirit))
  (bind _doorrotation (Timeline|DoorOpening Play)
    (:Update
      (Transformation|SetRelativeRotation (Variables|/Game/Blueprints/Interactables/BP_Door.BP_Door_C|GetDoor (Variables|Default|GetDoor)) (Math|Rotator|MakeRotator 0.0 0.0 _doorrotation) false false))
    (:Finished
      (Variables|/Game/Blueprints/Event/BP_EventDaddy.BP_EventDaddy_C|SetisActive (Variables|Default|GetNextEvent) true)
      (Actor|DestroyActor))))

(fn ConstructionScript
  (|CallParentFunction))
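; Test scare event that shifts two groups of spirits while the player is looking away.
; ThisEventBehavior retries every 0.2 seconds while the character's VisionCube overlaps DetectorBox or the event is inactive, ignoring triggers from the VisionCube itself.
; Once unseen and active, if the player overlaps Collider, it prints a debug "BOUH !", raises Spirits001List and lowers Spirits002List instantly.
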(event EventThisEventBehavior
  (params (OtherComp :type Primitive%20Component%20Object%20Reference))
  (bind _asbp_played_character (Utilities|Casting|CastToBP_PlayedCharacter (Game|GetPlayerCharacter 0)))
  (if (!= OtherComp (Variables|/Game/Blueprints/BP_PlayedCharacter.BP_PlayedCharacter_C|GetVisionCube _asbp_played_character))
    (if (Class|PrimitiveComponent|IsOverlappingComponent (Variables|/Game/Blueprints/BP_PlayedCharacter.BP_PlayedCharacter_C|GetVisionCube _asbp_played_character) (Variables|Default|GetDetectorBox))
      (Utilities|FlowControl|Delay 0.2 :!label _label)
      (CallFunction|ThisEventBehavior)
      (elif (Variables|Default|GetisActive)
        (if (Collision|IsOverlappingActor (Variables|Default|GetCollider) (Game|GetPlayerCharacter 0) :!class /Script/Engine.PrimitiveComponent)
          (Development|PrintString "BOUH !")
          (for _array_element (Variables|Default|GetSpirits001List)
            (Transformation|SetActorLocation _array_element (+ (Transformation|GetActorLocation _array_element) "0, 0,300.000000") false false))
          (for _array_element_2 (Variables|Default|GetSpirits002List)
            (Transformation|SetActorLocation _array_element_2 (+ (Transformation|GetActorLocation _array_element_2) "0, 0,-200.000000") false false)))
        (else
          (goto _label))))))

(fn ConstructionScript
  (|CallParentFunction))
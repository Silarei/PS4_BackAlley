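; BP_ThirdEventTest is a scripted event in an event chain, triggered by the player but ignoring their VisionCube.
; It retries every 0.2 seconds while inactive, or while the player overlaps its collider and the Nail still exists.
; Once the Nail is gone, it makes spirits disappear, alters lights, rotates two doors and destroys the first event.
; It then activates the next event and destroys itself.
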(event EventThisEventBehavior
  (params (OtherComp :type Primitive%20Component%20Object%20Reference))
  (bind _asbp_played_character (Utilities|Casting|CastToBP_PlayedCharacter (Game|GetPlayerCharacter 0)))
  (if (!= OtherComp (Variables|/Game/Blueprints/BP_PlayedCharacter.BP_PlayedCharacter_C|GetVisionCube _asbp_played_character))
    (if (Variables|Default|GetisActive)
      (if (Collision|IsOverlappingActor (Variables|Default|GetCollider) (Game|GetPlayerCharacter 0) :!class /Script/Engine.PrimitiveComponent)
        (Utilities|IsValid (Variables|Default|GetNail)
          (:Is%20Valid
            (Utilities|FlowControl|Delay 0.2 :!label _label)
            (CallFunction|ThisEventBehavior))
          (:Is%20Not%20Valid
            (for _array_element (Variables|Default|GetSpiritsList)
              (Default|Disappear _array_element))
            (for _array_element_2 (Variables|Default|GetLightsToTurnOff)
              (Rendering|SetVisibility (Variables|/Script/Engine.Light|GetLightComponent _array_element_2) false false))
            (Actor|DestroyActor (Variables|Default|GetFirstEvent))
            (for _array_element_3 (Variables|Default|GetLightsToTurnDown)
              (Class|LightComponent|SetTemperature (Variables|/Script/Engine.Light|GetLightComponent _array_element_3) 9e+03)
              (Rendering|Components|Light|SetIntensity (Variables|/Script/Engine.Light|GetLightComponent _array_element_3) 2.0))
            (Transformation|SetRelativeRotation (Variables|/Game/Blueprints/BP_Door.BP_Door_C|GetDoor (Variables|Default|GetDoor)) "0,100.000000, 0" false false)
            (Transformation|SetRelativeRotation (Variables|/Game/Blueprints/BP_Door.BP_Door_C|GetDoor (Variables|Default|GetDoorToOpen)) "0,40.000000, 0" false false)
            (Variables|/Game/Blueprints/Event/BP_EventTest.BP_EventTest_C|SetisActive (Variables|Default|GetNextEvent) true)
            (Actor|DestroyActor))))
      (else
        (goto _label)))))

(fn ConstructionScript
  (|CallParentFunction))
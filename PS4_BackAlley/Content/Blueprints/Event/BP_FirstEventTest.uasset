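; A scripted event Blueprint that changes a room while the player is not looking at its door.
; ThisEventBehavior re-runs itself every 0.2 seconds until the player character's VisionCube no longer overlaps the Door and the player overlaps the Collider.
; It then resets the door rotation, moves the Wall, turns on the room light, activates SecondEvent and destroys the Collider.
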(event EventThisEventBehavior
  (params (OtherComp :type Primitive%20Component%20Object%20Reference))
  (bind _asbp_played_character (Utilities|Casting|CastToBP_PlayedCharacter (Game|GetPlayerCharacter 0)))
  (if (Collision|IsOverlappingActor (Variables|/Game/Blueprints/BP_PlayedCharacter.BP_PlayedCharacter_C|GetVisionCube _asbp_played_character) (Variables|Default|GetDoor) :!class /Script/Engine.PrimitiveComponent)
    (Utilities|FlowControl|Delay 0.2 :!label _label)
    (CallFunction|ThisEventBehavior OtherComp)
    (elif (Collision|IsOverlappingActor (Variables|Default|GetCollider) (Game|GetPlayerCharacter 0) :!class /Script/Engine.PrimitiveComponent)
      (Transformation|SetRelativeRotation (Variables|/Game/Blueprints/Interactables/BP_Door.BP_Door_C|GetDoor (Variables|Default|GetDoor)) "0, 0, 0" false false)
      (Transformation|SetRelativeLocation (Variables|Default|GetWall) "0,-720.000000,133.000000" false false)
      (Rendering|SetVisibility (Variables|/Script/Engine.PointLight|GetPointLightComponent (Variables|Default|GetLightRoomEvent)) true false)
      (Variables|/Game/Blueprints/Event/BP_EventDaddy.BP_EventDaddy_C|SetisActive (Variables|Default|GetSecondEvent) true)
      (Components|DestroyComponent (Variables|Default|GetCollider))
      (else
        (goto _label)))))

(fn ConstructionScript
  (|CallParentFunction))
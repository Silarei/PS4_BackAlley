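; BP_Puke is a cleanable puke decal that a mop wipes away.
; BeginPlay gives the decal a dynamic material, and each overlap of its Box by a mop-interface actor while active lowers the material's opacity a step.
; When the opacity is used up, it notifies its Elevator that the puke is cleaned and destroys itself.
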(event OnComponentBeginOverlap(Box)
  (params (OverlappedComponent :type Primitive%20Component%20Object%20Reference) (OtherActor :type Actor%20Object%20Reference) (OtherComp :type Primitive%20Component%20Object%20Reference) (OtherBodyIndex :type Integer) (bFromSweep :type Boolean) (SweepResult :type Hit%20Result%20Structure%20%28by%20ref%29))
  (if (Variables|Default|GetIsActive)
    (Utilities|Casting|CastToBP_I_Mop OtherActor)
    (bind _output_get (Variables|Default|SetMatOpacity (- (Variables|Default|GetMatOpacity) 0.2)))
    (Rendering|Material|SetScalarParameterValue (Variables|Default|GetPukeMat) "Opacity" _output_get :!class /Script/Engine.MaterialInstanceDynamic)
    (if (<= (Variables|Default|GetMatOpacity) 0.0)
      (CallFunction|LaunchEvent))))

(event Custom|LaunchEvent
  (Default|OnPukeCleaned (Variables|Default|GetElevator))
  (Actor|DestroyActor))

(event EventBeginPlay
  (bind _returnvalue (Rendering|Material|CreateDynamicMaterialInstance (Variables|Decal|GetDecal) :!class /Script/Engine.DecalComponent))
  (bind _output_get (Variables|Default|SetPukeMat _returnvalue))
  (Rendering|Components|Decal|SetDecalMaterial (Variables|Decal|GetDecal) _output_get))

(event EventTick
  (params (DeltaSeconds :type Float%20%28single-precision%29)))

(fn ConstructionScript)
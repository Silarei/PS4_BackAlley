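; BP_Interactable is an interactable object with selected and unselected states and empty press and release events.
; It caches the main player controller at BeginPlay and reports itself as the selected interactable, clearing that on deselection.
; Selection binds event delegates to the controller's interact input and swaps the mesh material.
; Deselection unbinds them, restores the material and calls the release event, so an interaction ends with the selection.
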(event Custom|SetInteractable
  (params (CurrentlySelected :type BP%20Interactable%20Object%20Reference))
  (Default|SetSelectedInteractable (Variables|Default|GetMain%20Player%20Controller) CurrentlySelected))

(event Custom|InterractPressed)

(event Custom|InterractReleased)

(event EventBeginPlay
  (Variables|Default|SetMain%20Player%20Controller (CallFunction|GetMainPlayerController)))

(fn ConstructionScript)

(fn OnSelected
  (Default|BindOncetoInteract (Variables|Default|GetMain%20Player%20Controller) (EventDispatchers|CreateEvent :!event Custom|InterractPressed) (EventDispatchers|CreateEvent :!event Custom|InterractReleased))
  (CallFunction|SetInteractable self)
  (Rendering|Material|SetMaterial (Variables|Default|GetStaticMesh) 0 "/Game/Materials/Temp/M_SelectedMaterial.M_SelectedMaterial"))

(fn OnUnselected
  (Default|UnbindAllfromInteract (Variables|Default|GetMain%20Player%20Controller))
  (CallFunction|SetInteractable)
  (Rendering|Material|SetMaterial (Variables|Default|GetStaticMesh) 0 "/Game/Materials/Temp/M_UnselectedMaterial.M_UnselectedMaterial")
  (CallFunction|InterractReleased))
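; Interactable electric panel with a door and a set of switch buttons that can be flipped back once.
; BeginPlay gathers four button components into an array.
; AdditionalInteraction counts interactions and, from the second one on, calls SwitchElectricity if the door's yaw shows it is open far enough.
; SwitchElectricity mirrors each button by negating its relative roll, with the SwitchedBack flag preventing a repeat.
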(event Custom|SwitchElectricity
  (if (not (Variables|Default|GetSwitchedBack))
    (for _array_element (Variables|Default|GetButtons)
      (Transformation|SetRelativeRotation _array_element (Math|Rotator|MakeRotator (* (.Roll (Math|Rotator|BreakRotator (Variables|/Script/Engine.SceneComponent|GetRelativeRotation _array_element))) -1.0) (.Pitch (Math|Rotator|BreakRotator (Variables|/Script/Engine.SceneComponent|GetRelativeRotation _array_element))) (.Yaw (Math|Rotator|BreakRotator (Variables|/Script/Engine.SceneComponent|GetRelativeRotation _array_element)))) false false)
      (Variables|Default|SetSwitchedBack true))))

(event EventBeginPlay
  (|CallParentFunction)
  (Utilities|Array|Add (Variables|Default|GetButtons) (Variables|Default|GetButtons1))
  (Utilities|Array|Add (Variables|Default|GetButtons) (Variables|Default|GetButtons2))
  (Utilities|Array|Add (Variables|Default|GetButtons) (Variables|Default|GetButtons4))
  (Utilities|Array|Add (Variables|Default|GetButtons) (Variables|Default|GetButtons5)))

(event Collision|EventActorBeginOverlap
  (params (OtherActor :type Actor%20Object%20Reference)))

(event EventTick
  (params (DeltaSeconds :type Float%20%28single-precision%29))
  (|CallParentFunction DeltaSeconds) ; This node is disabled and will not be called.\nDrag off pins to build functionality.
)

(fn ConstructionScript
  (|CallParentFunction))

(fn AdditionalInteraction
  (Variables|Default|SetInteractionCount (+ (Variables|Default|GetInteractionCount) 1))
  (if (and (>= (.Yaw (Math|Rotator|BreakRotator (Variables|/Script/Engine.SceneComponent|GetRelativeRotation (Variables|Default|GetDoor)))) 5e+01) (>= (Variables|Default|GetInteractionCount) 2))
    (CallFunction|SwitchElectricity)))
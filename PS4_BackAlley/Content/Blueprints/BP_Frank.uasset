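; BP_Frank is the Blueprint for the character Frank, who carries a shovel and makes footstep sounds while moving.
; On BeginPlay it spawns a scaled-down BP_FrankShovel and attaches it to the mesh at ShovelSocket.
; Tick calls Footstep, which plays FootSteps above a small velocity threshold, using a DoOnce reset by a Delay to limit it to once per second.
; A Running event sets the walk speed, with nothing here to restore it.
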(event Custom|Running
  (Variables|/Script/Engine.CharacterMovementComponent|SetMaxWalkSpeed (Variables|Character|GetCharacterMovement) 3.5e+02))

(event Custom|Footstep
  (if (> (Math|Vector|VectorLength (Transformation|GetVelocity)) 5e+01)
    (Utilities|FlowControl|DoOnce false :!label _label
      (:Completed
        (Audio|Components|Audio|Play (Variables|Default|GetFootSteps) 0.0)
        (Utilities|FlowControl|Delay 1.0)
        (goto _label Reset)))))

(event EventBeginPlay
  (bind _returnvalue (Game|SpawnActorfromClass "/Game/Blueprints/EndSequence/BP_FrankShovel.BP_FrankShovel_C" (Math|Transform|MakeTransform "0, 0, 0" "0, 0, 0" "0.800000,0.800000,0.800000") "Undefined" 0 0))
  (bind _output_get (Variables|Default|SetShovel _returnvalue))
  (Transformation|AttachComponentToComponent _output_get (Variables|Character|GetMesh) "ShovelSocket" "KeepRelative" "KeepRelative" "KeepWorld" true))

(event EventTick
  (params (DeltaSeconds :type Float%20%28single-precision%29))
  (CallFunction|Footstep))

(fn ConstructionScript)